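; Default level data config that builds procedural walls for generated levels when its CreateWall event fires.
; It spawns a BP_Proc_Wall through the level data and places it at the given offset.
; The vertices become a zero-tangent, straight-segment horizontal spline at the wall offset height, and a two-point vertical spline sets the wall height.
; The wall's Generate call then builds it from both splines.
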(event `self.CreateWall`
  (params (aLevelData :type "LevelData Object Reference") (someVertices :type "Array of Vector2D Structure (by ref)") (anOffset :type "Vector Structure (by ref)") (aWallOffset :type "Float (single-precision)") (aWallHeight :type "Float (single-precision)"))
  (bind _returnvalue (`LevelData.SpawnGeneratedActor` aLevelData "/Game/Props/Procedural/Walls/BP_Proc_Wall.BP_Proc_Wall_C"))
  (bind _asbp_proc_wall (cast `/Game/Props/Procedural/Walls/BP_Proc_Wall` _returnvalue))
  (bind _output_get (set `self.Wall` _asbp_proc_wall))
  (`Actor.K2_SetActorLocation` _output_get anOffset false false)
  (`|ExecutionSequence`
    (:`then_0`
      (`self.CreateWallHorizontalSpline` someVertices aWallOffset))
    (:`then_1`
      (`self.CreateWallVerticalSpline` aWallHeight))
    (:`then_2`
      (`/Game/Props/Procedural/Helpers/BP_Proc_Mesh.Generate` (`self.Wall`)))))

(fn `CreateWallHorizontalSpline`
  (params (Vertices :type "Array of Vector2D Structure (by ref)") (WallOffset :type "Float (single-precision)"))
  (locals (Points :type "Array of Vector Structure"))
  (bind _spline (`/Game/Props/Procedural/Helpers/BP_Proc_SplineMesh.Spline` (`self.Wall`)))
  (`KismetArrayLibrary.Array_Clear` (`local.Points`))
  (for _array_element Vertices
    (bind (_x _y) (`KismetMathLibrary.BreakVector2D` _array_element))
    (`KismetArrayLibrary.Array_Add` (`local.Points`) (`KismetMathLibrary.MakeVector` _x _y WallOffset)))
  (`SplineComponent.SetSplinePoints` _spline (`local.Points`) "Local" false)
  (for _index (range (`SplineComponent.GetNumberOfSplinePoints` _spline))
    (`SplineComponent.SetTangentAtSplinePoint` _spline _index (`KismetMathLibrary.MakeVector` 0.0) "Local" false))
  (`SplineComponent.UpdateSpline` (`/Game/Props/Procedural/Helpers/BP_Proc_SplineMesh.Spline` (`self.Wall`))))

(fn `CreateWallVerticalSpline`
  (params (WallHeight :type "Float (double-precision)"))
  (locals (Points :type "Array of Vector Structure"))
  (bind _points (`local.Points`))
  (`KismetArrayLibrary.Array_Clear` _points)
  (`KismetArrayLibrary.Array_Add` _points (`KismetMathLibrary.MakeVector` 0.0))
  (`KismetArrayLibrary.Array_Add` _points (`KismetMathLibrary.MakeVector` 0.0 0.0 WallHeight))
  (`SplineComponent.SetSplinePoints` (`/Game/Props/Procedural/Walls/BP_Proc_Wall.VerticalSpline` (`self.Wall`)) (`local.Points`) "Local" true))