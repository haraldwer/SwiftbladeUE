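; Procedural level-end actor that builds a wall at its own transform when its end location is set.
; It destroys previously spawned actors, then spawns a BP_Proc_Wall shaped by fixed horizontal and vertical splines.
; A hidden, query-only overlap sphere mesh is registered in the wall's SphereOverlaps before the wall generates.
; All spawns go through a helper that owns and tracks them for cleanup.
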(event `self.OnEndLocationSet`
  (`self.ClearSpawnedActors`)
  (bind _actor (`self.CreateActor` "/Game/Props/Procedural/Walls/BP_Proc_Wall.BP_Proc_Wall_C"))
  (bind _asbp_proc_wall (cast `/Game/Props/Procedural/Walls/BP_Proc_Wall` _actor))
  (`SplineComponent.SetSplinePoints` (`/Game/Props/Procedural/Helpers/BP_Proc_SplineMesh.Spline` _asbp_proc_wall) (`|MakeArray` (-3000.0 0.0 0.0) (3000.0 0.0 0.0) :!type "Vector Structure") "Local" true)
  (`SplineComponent.SetSplinePoints` (`/Game/Props/Procedural/Walls/BP_Proc_Wall.VerticalSpline` _asbp_proc_wall) (`|MakeArray` (0.0 0.0 -2000.0) (0.0 0.0 4000.0) :!type "Vector Structure") "Local" true)
  (bind _actor_2 (`self.CreateActor` "/Script/Engine.StaticMeshActor"))
  (bind _asstatic_mesh_actor (cast `StaticMeshActor` _actor_2))
  (bind _staticmeshcomponent (`StaticMeshActor.StaticMeshComponent` _asstatic_mesh_actor))
  (`StaticMeshComponent.SetStaticMesh` _staticmeshcomponent "/Engine/BasicShapes/Sphere.Sphere")
  (`PrimitiveComponent.SetCollisionResponseToAllChannels` _staticmeshcomponent "ECR_Overlap")
  (`PrimitiveComponent.SetCollisionEnabled` _staticmeshcomponent "QueryOnly")
  (`self.SetActorHiddenInGame` _asstatic_mesh_actor true)
  (`KismetArrayLibrary.Array_Add` (`/Game/Props/Procedural/Helpers/BP_Proc_SplineMesh.SphereOverlaps` _asbp_proc_wall) _asstatic_mesh_actor)
  (`/Game/Props/Procedural/Helpers/BP_Proc_Mesh.Generate` _asbp_proc_wall))

(fn `ClearSpawnedActors`
  (for _array_element (`self.SpawnedActors`)
    (`self.K2_DestroyActor` _array_element))
  (`KismetArrayLibrary.Array_Clear` (`self.SpawnedActors`)))

(fn `CreateActor`
  (params (Class :type "Actor Class Reference"))
  (returns (Actor :type "Actor Object Reference"))
  (bind _returnvalue (`|SpawnActorFromClass` Class (`self.GetTransform`) "AlwaysSpawn" "OverrideRootScale" self null))
  (`KismetArrayLibrary.Array_Add` (`self.SpawnedActors`) _returnvalue)
  (return _returnvalue))

(fn `UserConstructionScript`
  (`parent.UserConstructionScript`))