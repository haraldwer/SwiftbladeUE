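; Procedural level section component that builds a room wall as a spawned ProcSplineMesh actor.
; CreateWall spawns WallClass through the generator, then shapes the actor's two splines before calling GenerateMesh.
; The first spline traces the given vertices at the ground offset, with zeroed tangents for straight segments.
; The second is a vertical line sized as a percentage of ceiling height.
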(event `self.CreateWall`
  (params (aGenerator :type "SectionGenerator Object Reference") (aArray :type "Array of Vector2D Structure (by ref)") (anIndex :type Integer) (aGroundOffset :type "Float (single-precision)") (aCeilHeight :type "Float (single-precision)"))
  (bind _returnvalue (`SectionGenerator.SpawnGeneratedActor` aGenerator (`self.WallClass`) (`KismetMathLibrary.MakeTransform` (0.0 0.0 0.0))))
  (set `self.Wall` _returnvalue)
  (`|ExecutionSequence`
    (:`then_0`
      (`self.CreateHorizontalSpline` aArray aGroundOffset))
    (:`then_1`
      (`self.CreateVerticalSpline` (* aCeilHeight (/ (`self.RoomHeightPercentage`) 100.0))))
    (:`then_2`
      (bind _asproc_spline_mesh (cast `ProcSplineMesh` (`self.Wall`)))
      (`ProcSplineMesh.GenerateMesh` _asproc_spline_mesh))))

(fn `CreateHorizontalSpline`
  (params (Vertices :type "Array of Vector2D Structure (by ref)") (WallOffset :type "Float (single-precision)"))
  (locals (Points :type "Array of Vector Structure") (Spline :type "SplineComponent Object Reference"))
  (bind _spline (`local.Spline`))
  (bind _spline_2 (`local.Spline`))
  (bind _asproc_spline_mesh (cast `ProcSplineMesh` (`self.Wall`)))
  (bind _output_get (set `local.Spline` (`ProcSplineMesh.GetSpline` _asproc_spline_mesh 0)))
  (`/Engine/EditorBlueprintResources/StandardMacros.IsValid` _output_get
    (:`Is Valid`
      (`KismetArrayLibrary.Array_Clear` (`local.Points`))
      (for _array_element Vertices
        (bind (_x _y) (`KismetMathLibrary.BreakVector2D` _array_element))
        (`KismetArrayLibrary.Array_Add` (`local.Points`) (`KismetMathLibrary.MakeVector` _x _y WallOffset)))
      (`SplineComponent.SetSplinePoints` _spline (`local.Points`) "Local" false)
      (for _index (range (`SplineComponent.GetNumberOfSplinePoints` _spline))
        (`SplineComponent.SetTangentAtSplinePoint` _spline_2 _index (`KismetMathLibrary.MakeVector` 0.0) "Local" false)
        (`SplineComponent.SetScaleAtSplinePoint` _spline_2 _index (`KismetMathLibrary.Vector_One`) false))
      (`SplineComponent.UpdateSpline` _spline_2))))

(fn `CreateVerticalSpline`
  (params (WallHeight :type "Float (double-precision)"))
  (locals (Points :type "Array of Vector Structure"))
  (bind _points (`local.Points`))
  (`KismetArrayLibrary.Array_Clear` _points)
  (`KismetArrayLibrary.Array_Add` _points (`KismetMathLibrary.MakeVector` 0.0))
  (`KismetArrayLibrary.Array_Add` _points (`KismetMathLibrary.MakeVector` 0.0 0.0 WallHeight))
  (bind _asproc_spline_mesh (cast `ProcSplineMesh` (`self.Wall`)))
  (bind _returnvalue (`ProcSplineMesh.GetSpline` _asproc_spline_mesh 1))
  (`/Engine/EditorBlueprintResources/StandardMacros.IsValid` _returnvalue
    (:`Is Valid`
      (`SplineComponent.SetSplinePoints` _returnvalue (`local.Points`) "Local" true))))