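; Procedural room section component that creates the ground mesh floor for a generated room.
; When a room is populated, it asks the generator to spawn a FloorType actor at the origin and casts it to BP_Proc_Floor.
; It rebuilds that floor's spline from the room's 2D vertices, raised to the room's ground offset, then calls Generate on the floor.
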(event `self.BPPopulateRoom`
  (params (aGenerator :type "SectionGenerator Object Reference") (aSection :type "ProcSection Structure (by ref)") (aRoom :type "ProcRoom Structure (by ref)"))
  (bind _returnvalue (`GeneratorBase.SpawnGeneratedActor` aGenerator (`self.FloorType`) (`KismetMathLibrary.MakeTransform` (0.0 0.0 0.0))))
  (bind _asbp_proc_floor (cast `/Game/Rooms/Building/Floors/BP_Proc_Floor` _returnvalue))
  (`self.SetFloorSpline` _asbp_proc_floor aRoom))

(fn `SetFloorSpline`
  (params (Floor :type "/Game/Rooms/Building/Floors/BP_Proc_Floor Object Reference") (ProcRoom :type "ProcRoom Structure (by ref)"))
  (locals (Points :type "Array of SplinePoint Structure") (Count :type "Float (double-precision)"))
  (bind (_index _location _center _vertices _edges _walls _path _radius _groundoffset) (break `ProcRoom` ProcRoom))
  (bind _spline (`/Game/Rooms/Building/Floors/BP_Proc_Floor.Spline` Floor))
  (`KismetArrayLibrary.Array_Clear` (`local.Points`))
  (set `local.Count` 0.0)
  (for _array_element _vertices
    (bind _output_get (set `local.Count` (+ (`local.Count`) 1.0)))
    (`KismetArrayLibrary.Array_Add` (`local.Points`) (make `SplinePoint` _output_get (`KismetMathLibrary.Conv_Vector2DToVector` _array_element _groundoffset) (0.0 0.0 0.0) (0.0 0.0 0.0) (struct) (1.0 1.0 1.0) "Linear")))
  (`SplineComponent.ClearSplinePoints` _spline false)
  (`SplineComponent.AddPoints` _spline (`local.Points`) true)
  (`/Game/Procedural/BP_Proc_Mesh.Generate` Floor))