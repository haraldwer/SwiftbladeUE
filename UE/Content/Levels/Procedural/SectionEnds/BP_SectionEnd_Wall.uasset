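; BP_SectionEnd_Wall is a procedural level section end that shapes a procedural wall hosted in a child actor component.
; When its location is set, it rewrites the wall's two splines into straight local lines, one horizontal along X and one vertical along Z.
; It then adds itself to the wall's SphereOverlaps and triggers the wall's mesh generation.
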(event `self.OnLocationSet`
  (bind _asbp_proc_wall (cast `/Game/Props/Procedural/Walls/BP_Proc_Wall` (`ChildActorComponent.ChildActor` (`self.ProcWall`))))
  (`|ExecutionSequence`
    (:`then_0`
      (bind _returnvalue (`/Game/Props/Procedural/Helpers/BP_Proc_SplineMesh.GetSpline` _asbp_proc_wall 0))
      (`/Engine/EditorBlueprintResources/StandardMacros.IsValid` _returnvalue
        (:`Is Valid`
          (`SplineComponent.SetSplinePoints` _returnvalue (`|MakeArray` (-5000.0 0.0 0.0) (5000.0 0.0 0.0) :!type "Vector Structure") "Local" true))))
    (:`then_1`
      (bind _returnvalue_2 (`/Game/Props/Procedural/Helpers/BP_Proc_SplineMesh.GetSpline` _asbp_proc_wall 1))
      (`/Engine/EditorBlueprintResources/StandardMacros.IsValid` _returnvalue_2
        (:`Is Valid`
          (`SplineComponent.SetSplinePoints` _returnvalue_2 (`|MakeArray` (0.0 0.0 -3000.0) (0.0 0.0 3000.0) :!type "Vector Structure") "Local" true))))
    (:`then_2`
      (`KismetArrayLibrary.Array_Add` (`/Game/Props/Procedural/Helpers/BP_Proc_SplineMesh.SphereOverlaps` _asbp_proc_wall) self)
      (message `ProcSplineMesh.GenerateMesh` _asbp_proc_wall))))

(fn `UserConstructionScript`
  (`parent.UserConstructionScript`))