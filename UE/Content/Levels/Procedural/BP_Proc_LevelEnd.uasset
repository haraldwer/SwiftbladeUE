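; BP_Proc_LevelEnd builds the end of a procedurally generated level as a wall with a hole marker.
; When the end location is set, it asks the generator to spawn a BP_Proc_Wall at its transform and gives it fixed horizontal and vertical splines.
; It also spawns a hidden, query-only overlap sphere scaled by HoleScale and registers it in the wall's SphereOverlaps before calling Generate.
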(event `self.OnEndLocationSet`
  (params (aGenerator :type "SectionGenerator Object Reference"))
  (bind _returnvalue (`SectionGenerator.SpawnGeneratedActor` aGenerator (`self.Wall`) (`self.GetTransform`)))
  (bind _asbp_proc_wall (cast `/Game/Props/Procedural/Walls/BP_Proc_Wall` _returnvalue))
  (`SplineComponent.SetSplinePoints` (`/Game/Props/Procedural/Helpers/BP_Proc_SplineMesh.Spline` _asbp_proc_wall) (`|MakeArray` (-3000.0 0.0 0.0) (3000.0 0.0 0.0) :!type "Vector Structure") "Local" true)
  (`SplineComponent.SetSplinePoints` (`/Game/Props/Procedural/Walls/BP_Proc_Wall.VerticalSpline` _asbp_proc_wall) (`|MakeArray` (0.0 0.0 -4000.0) (0.0 0.0 2000.0) :!type "Vector Structure") "Local" true)
  (bind _returnvalue_2 (`SectionGenerator.SpawnGeneratedActor` aGenerator (`self.Hole`) (`self.GetTransform`)))
  (bind _asstatic_mesh_actor (cast `StaticMeshActor` _returnvalue_2))
  (`self.SetActorScale3D` _asstatic_mesh_actor (`self.HoleScale`))
  (bind _staticmeshcomponent (`StaticMeshActor.StaticMeshComponent` _asstatic_mesh_actor))
  (`SceneComponent.SetMobility` _staticmeshcomponent "Movable")
  (`StaticMeshComponent.SetStaticMesh` _staticmeshcomponent "/Engine/BasicShapes/Sphere.Sphere")
  (`PrimitiveComponent.SetCollisionResponseToAllChannels` _staticmeshcomponent "ECR_Overlap")
  (`PrimitiveComponent.SetCollisionEnabled` _staticmeshcomponent "QueryOnly")
  (`self.SetActorHiddenInGame` _asstatic_mesh_actor true)
  (`KismetArrayLibrary.Array_Add` (`/Game/Props/Procedural/Helpers/BP_Proc_SplineMesh.SphereOverlaps` _asbp_proc_wall) _asstatic_mesh_actor)
  (`/Game/Props/Procedural/Helpers/BP_Proc_Mesh.Generate` _asbp_proc_wall))

(fn `UserConstructionScript`
  (`parent.UserConstructionScript`))