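; Arena generator component that builds the procedural ground floor for an arena subdivision.
; On populate, it spawns the configured floor actor through the generator and casts it to BP_Proc_Floor.
; It converts the subdivision's 2D vertices into spline points at the subdivision's height, replaces the floor's spline with them, then triggers the floor's generation.
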(event `self.BPPopulate`
  (params (aArenaGenerator :type "ArenaGenerator Object Reference") (aLayer :type "ArenaLayer Structure (by ref)") (aSection :type "ArenaSection Structure (by ref)") (aSubdivision :type "ArenaSubdivision Structure (by ref)"))
  (bind _returnvalue (`GeneratorBase.SpawnGeneratedActor` aArenaGenerator (`self.FloorType`) (`KismetMathLibrary.MakeTransform` (0.0 0.0 0.0))))
  (bind _asbp_proc_floor (cast `/Game/Rooms/Building/Floors/BP_Proc_Floor` _returnvalue))
  (`self.SetFloorSpline` aSubdivision _asbp_proc_floor))

(fn `SetFloorSpline`
  (params (Subdivision :type "ArenaSubdivision Structure (by ref)") (Floor :type "/Game/Rooms/Building/Floors/BP_Proc_Floor Object Reference"))
  (locals (Points :type "Array of SplinePoint Structure") (Count :type "Float (double-precision)"))
  (bind (_height _startangle _endangle _vertices) (break `ArenaSubdivision` Subdivision))
  (bind _spline (`/Game/Rooms/Building/Floors/BP_Proc_Floor.Spline` Floor))
  (`KismetArrayLibrary.Array_Clear` (`local.Points`))
  (set `local.Count` 0.0)
  (for _array_element _vertices
    (bind _output_get (set `local.Count` (+ (`local.Count`) 1.0)))
    (`KismetArrayLibrary.Array_Add` (`local.Points`) (make `SplinePoint` _output_get (`KismetMathLibrary.Conv_Vector2DToVector` _array_element _height) (0.0 0.0 0.0) (0.0 0.0 0.0) (struct) (1.0 1.0 1.0) "Linear")))
  (`SplineComponent.ClearSplinePoints` _spline false)
  (`SplineComponent.AddPoints` _spline (`local.Points`) true)
  (`/Game/Procedural/BP_Proc_Mesh.Generate` Floor))