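; BP_Proc_Vines procedurally grows a branching vine from the actor's location along its forward vector in the construction script.
; CreateBranch recurses into one main branch and random sub-branches, picking random step lengths and directions within a split-angle cone.
; Target lengths and a shared iteration cap bound the growth.
; Each segment becomes a scaled, oriented mesh instance; AdjustDirection is a stub whose result is unused.
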(fn `AddMesh`
  (params (Position :type "Vector Structure") (Direction :type "Vector Structure") (CurrentBranchLength :type "Float (double-precision)"))
  (bind _direction (`local.Direction`))
  (bind _vineradius (`self.VineRadius`))
  (bind _component (`self.GetMeshComponent` (`self.Mesh`)))
  (`InstancedStaticMeshComponent.AddInstance` _component (`KismetMathLibrary.MakeTransform` (+ (`local.Position`) (* (* (`local.CurrentBranchLength`) 0.5) _direction)) (`KismetMathLibrary.FindLookAtRotation` (`KismetMathLibrary.MakeVector` 0.0) _direction) (`self.AdjustScaleForMeshSize` (`self.Mesh`) (`KismetMathLibrary.MakeVector` (`local.CurrentBranchLength`) _vineradius _vineradius))) false))

(fn `AdjustDirection`
  (params (Direction :type "Vector Structure") (Position :type "Vector Structure") (CurrentLength :type "Float (double-precision)"))
  (returns (Result :type "Vector Structure") (Hit :type Boolean))
  (return (0.0 0.0 0.0) false))

(fn `CreateBranch`
  (params (Position :type "Vector Structure") (Direction :type "Vector Structure") (IsMain :type Boolean) (CurrentVineLength :type "Float (double-precision)") (TargetVineLength :type "Float (double-precision)") (CurrentBranchLength :type "Float (double-precision)"))
  (locals (CachedBranchLength :type "Float (double-precision)"))
  (if (< (`self.Iterations`) (`self.MaxIterations`))
    (set `self.Iterations` (+ (`self.Iterations`) 1))
    (`self.AdjustDirection` (0.0 0.0 0.0))
    (`self.AddMesh` (`local.Position`) (`local.Direction`) (`local.CurrentBranchLength`))
    (if (< (`local.CurrentVineLength`) (`local.TargetVineLength`))
      (`|ExecutionSequence`
        (:`then_0`
          (if (`local.IsMain`)
            (set `local.CachedBranchLength` (`KismetMathLibrary.RandomFloatInRange` (`self.MinStepLength`) (`self.MaxStepLength`)))
            (`self.CreateBranch` (+ (`local.Position`) (* (`local.Direction`) (`local.CurrentBranchLength`))) (`KismetMathLibrary.RandomUnitVectorInConeInDegrees` (`local.Direction`) (`self.SplitAngle`)) true (+ (`local.CurrentVineLength`) (`local.CurrentBranchLength`)) (`self.VineLength`) (`local.CachedBranchLength`))))
        (:`then_1`
          (for _ (range (+ (`KismetMathLibrary.FTrunc` (`KismetMathLibrary.RandomFloatInRange` (`self.MinSubBranches`) (`self.MaxSubBranches`))) 1))
            (set `local.CachedBranchLength` (`KismetMathLibrary.RandomFloatInRange` (`self.MinStepLength`) (`self.MaxStepLength`)))
            (`self.CreateBranch` (+ (`local.Position`) (* (`local.Direction`) (`local.CurrentBranchLength`))) (`KismetMathLibrary.RandomUnitVectorInConeInDegrees` (`local.Direction`) (`self.SplitAngle`)) false (+ (`local.CurrentVineLength`) (`local.CurrentBranchLength`)) (`KismetMathLibrary.RandomFloatInRange` 0.0 (`KismetMathLibrary.FMin` (`self.MaxBranchLength`) (- (`self.VineLength`) (`local.CurrentVineLength`)))) (`local.CachedBranchLength`))))))))

(fn `UserConstructionScript`
  (`self.CreateBranch` (`self.K2_GetActorLocation`) (`self.GetActorForwardVector`) true 0.0 (`self.VineLength`)))