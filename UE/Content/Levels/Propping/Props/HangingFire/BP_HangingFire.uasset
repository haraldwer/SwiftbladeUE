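; BP_HangingFire is a level prop that gives a hanging fire a gentle, irregular sway.
; Each Tick it accumulates a timer and samples 1D Perlin noise at two offset times to drive small roll and pitch angles.
; The scaled result sets the world rotation of WiggleRoot, with yaw held at zero.
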(event `self.ReceiveTick`
  (params (DeltaSeconds :type "Float (single-precision)"))
  (set `self.Timer` (+ DeltaSeconds (`self.Timer`)))
  (`SceneComponent.K2_SetWorldRotation` (`self.WiggleRoot`) (* (`KismetMathLibrary.MakeRotator` (`KismetMathLibrary.PerlinNoise1D` (`self.Timer`)) (`KismetMathLibrary.PerlinNoise1D` (+ (`self.Timer`) 100.0))) 2.0) false false))

(fn `UserConstructionScript`)