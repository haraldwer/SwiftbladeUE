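; Enemy Blueprint that plays a spawn-in effect when it enters the game.
; After the parent BeginPlay runs, it spawns a BP_Enemy_SpawnParticle actor at its own transform, then hides itself and pauses its tick and the MyBehaviour component's tick.
; A short fixed delay then reveals the enemy and resumes both ticks; collision is left untouched throughout.
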(event `self.ReceiveBeginPlay`
  (`parent.ReceiveBeginPlay`)
  (`self.ShowSpawnEffect`))

(event `ShowSpawnEffect`
  (`|SpawnActorFromClass` "/Game/Blueprints/Enemy/Spawning/BP_Enemy_SpawnParticle.BP_Enemy_SpawnParticle_C" (`self.GetTransform`) "AlwaysSpawn" "OverrideRootScale" null null)
  (`self.SetActorHiddenInGame` true)
  (`self.SetActorTickEnabled` false)
  (`ActorComponent.SetComponentTickEnabled` (`self.myBehaviour`) false)
  (`KismetSystemLibrary.Delay` 1.7)
  (`self.SetActorHiddenInGame` false)
  (`self.SetActorTickEnabled` true)
  (`ActorComponent.SetComponentTickEnabled` (`self.myBehaviour`) true))

(fn `UserConstructionScript`)