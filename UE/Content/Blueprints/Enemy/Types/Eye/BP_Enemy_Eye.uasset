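; Eye enemy Blueprint that adds a wandering, randomized tumble to its three ring components.
; BeginPlay randomly seeds a stream and draws a starting angular velocity for each ring.
; Every Tick, RotateRing nudges each velocity by a delta-scaled random rotation, slowly interpolates it toward zero, then applies it as world rotation.
; The velocity is written back by reference, so each ring drifts independently.
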(event `self.ReceiveBeginPlay`
  (bind _returnvalue (`KismetMathLibrary.MakeRotator` (`KismetMathLibrary.RandomFloatInRangeFromStream` -180.0 180.0 (`self.Random`)) (`KismetMathLibrary.RandomFloatInRangeFromStream` -180.0 180.0 (`self.Random`)) (`KismetMathLibrary.RandomFloatInRangeFromStream` -180.0 180.0 (`self.Random`))))
  (`parent.ReceiveBeginPlay`)
  (`KismetMathLibrary.SetRandomStreamSeed` (`self.Random`) (`KismetMathLibrary.RandomInteger` 9999999))
  (set `self.RingAngularVel_0` _returnvalue)
  (set `self.RingAngularVel_1` _returnvalue)
  (set `self.RingAngularVel_2` _returnvalue))

(event `self.ReceiveTick`
  (params (DeltaSeconds :type "Float (single-precision)"))
  (`self.Rotate Ring` DeltaSeconds (`self.Ring`) (`self.RingAngularVel_0`))
  (`self.Rotate Ring` DeltaSeconds (`self.Ring1`) (`self.RingAngularVel_1`))
  (`self.Rotate Ring` DeltaSeconds (`self.Ring2`) (`self.RingAngularVel_2`)))

(fn `Rotate Ring`
  (params (Delta :type "Float (double-precision)") (Ring :type "SceneComponent Object Reference") (Rotator :type "Rotator Structure (by ref)"))
  (`/Engine/EditorBlueprintResources/StandardMacros.IsValid` Ring
    (:`Is Valid`
      (`|VariableSetRef` Rotator (`KismetMathLibrary.RInterpTo` (`KismetMathLibrary.ComposeRotators` (* (`KismetMathLibrary.MakeRotator` (`KismetMathLibrary.RandomFloatInRangeFromStream` -180.0 180.0 (`self.Random`)) (`KismetMathLibrary.RandomFloatInRangeFromStream` -180.0 180.0 (`self.Random`)) (`KismetMathLibrary.RandomFloatInRangeFromStream` -180.0 180.0 (`self.Random`))) (* 1.0 Delta)) Rotator) (struct) Delta 0.05))
      (`SceneComponent.K2_AddWorldRotation` Ring (* Rotator Delta) false false))))

(fn `UserConstructionScript`
  (`parent.UserConstructionScript`))