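; Necromancer enemy Blueprint that fades a book light in while the enemy is in its attack state.
; BeginPlay creates a dynamic book-light material, passes the child components of SpawnLocations to the necromancer attack state and binds to behavior state changes.
; State changes toggle a show-book flag, and Tick eases the alpha of the pink light color toward it with FInterpTo.
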(event `self.ReceiveBeginPlay`
  (`parent.ReceiveBeginPlay`)
  (add `EnemyBehaviour.myOnBehaviourStateChanged` (`self.myBehaviour`) (`|CreateDelegate` :!event `OnStateChanged`))
  (bind _returnvalue (`PrimitiveComponent.CreateDynamicMaterialInstance` (`self.StaticMesh`) 0 "/Game/Materials/M_BookLight.M_BookLight" "MI_Enemy_Necromancer_BookLight"))
  (set `self.BookLight` _returnvalue)
  (set `EnemyStateAttackNecromancer.mySpawnLocations` (`SceneComponent.GetChildrenComponents` (`self.SpawnLocations`) false) (`self.EnemyStateAttackNecromancer`)))

(event `OnStateChanged`
  (params (aState :type "EnemyBaseState Object Reference"))
  (set `self.bShowBook` (== aState (`self.EnemyStateAttackNecromancer`))))

(event `self.ReceiveTick`
  (params (DeltaSeconds :type "Float (single-precision)"))
  (bind _output_get (set `self.BookAlpha` (`KismetMathLibrary.FInterpTo` (`self.BookAlpha`) (`KismetMathLibrary.Conv_BoolToDouble` (`self.bShowBook`)) DeltaSeconds 3.0)))
  (`MaterialInstanceDynamic.SetVectorParameterValue` (`self.BookLight`) "Color" (`KismetMathLibrary.MakeColor` 1.0 0.55 0.95 (* _output_get 0.5))))

(fn `UserConstructionScript`
  (`parent.UserConstructionScript`))