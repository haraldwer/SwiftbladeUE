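; BP_DeadlyComponent is an actor component that makes its owner lethal to FPCharacter actors.
; On BeginPlay it binds the owner's hit event, plus begin overlap unless OnlyOnHit is set.
; Hits are routed into the overlap handler, which casts the other actor to FPCharacter and calls Die with the component's object name.
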(event `self.ReceiveBeginPlay`
  (bind _returnvalue (`self.GetOwner`))
  (if (not (`self.OnlyOnHit`))
    (add `Actor.OnActorBeginOverlap` _returnvalue (delegate `OnOverlap`)))
  (add `Actor.OnActorHit` _returnvalue (delegate `OnHit`)))

(event `OnHit`
  (params (SelfActor :type "Actor Object Reference") (OtherActor :type "Actor Object Reference") (NormalImpulse :type "Vector Structure") (Hit :type "HitResult Structure (by ref)"))
  (`self.OnOverlap` null OtherActor))

(event `OnOverlap`
  (params (OverlappedActor :type "Actor Object Reference") (OtherActor :type "Actor Object Reference"))
  (bind _asfpcharacter (cast `FPCharacter` OtherActor))
  (`FPCharacter.Die` _asfpcharacter (`KismetSystemLibrary.GetObjectName` self)))