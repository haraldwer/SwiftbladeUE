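; Checkpoint crystal that reveals itself once enabled and plays a pickup effect when activated.
; While enabled, Tick eases a visibility value that drives a material parameter collection, Niagara scale, crystal rise and light intensity as the crystal spins.
; Activation shows the pickup effect, hides the crystal, then calls FinishActivate after short delays.
; Once activated, Tick also eases global time dilation toward zero, slowing the game.
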(event `self.ReceiveBeginPlay`
  (`KismetMaterialLibrary.SetScalarParameterValue` "/Game/Blueprints/Gameplay/Checkpoint/Param_Crystal.Param_Crystal" "Visibility"))

(event `self.ReceiveTick`
  (params (DeltaSeconds :type "Float (single-precision)"))
  (`|ExecutionSequence`
    (:`then_0`
      (if (`self.IsEnabled`)
        (bind _output_get (set `self.CrystalVisibility` (`KismetMathLibrary.FInterpTo` (`self.CrystalVisibility`) 1.0 DeltaSeconds 2.0)))
        (`KismetMaterialLibrary.SetScalarParameterValue` "/Game/Blueprints/Gameplay/Checkpoint/Param_Crystal.Param_Crystal" "Visibility" _output_get)
        (`SceneComponent.SetRelativeScale3D` (`self.NS_Crystal`) (`KismetMathLibrary.MakeVector` _output_get _output_get _output_get))
        (`SceneComponent.K2_SetRelativeRotation` (`self.Crystal`) (`KismetMathLibrary.ComposeRotators` (`KismetMathLibrary.MakeRotator` 0.0 0.0 (* DeltaSeconds 50.0)) (`SceneComponent.RelativeRotation` (`self.Crystal`))) false false)
        (`SceneComponent.K2_SetRelativeLocation` (`self.Crystal`) (`KismetMathLibrary.VLerp` (`SceneComponent.RelativeLocation` (`self.Start`)) (`SceneComponent.RelativeLocation` (`self.End`)) (`self.CrystalVisibility`)) false false)
        (`LightComponent.SetIntensity` (`self.PointLight`) (`KismetMathLibrary.Lerp` 0.0 500.0 (`self.CrystalVisibility`)))))
    (:`then_1`
      (if (`self.bActivated`)
        (`GameplayStatics.SetGlobalTimeDilation` (`KismetMathLibrary.FInterpTo` (`GameplayStatics.GetGlobalTimeDilation`) 0.0 DeltaSeconds 5.0))))))

(event `self.Activate`
  (params (anInstigator :type "FPController Object Reference"))
  (bind _ns_pickupcrystal (`self.NS_PickupCrystal`))
  (`SceneComponent.SetVisibility` _ns_pickupcrystal true false)
  (`ActorComponent.Activate` _ns_pickupcrystal true)
  (set `self.bActivated` true)
  (`KismetSystemLibrary.Delay` 0.1)
  (`SceneComponent.SetVisibility` (`self.Crystal`) false false)
  (`SceneComponent.SetVisibility` (`self.NS_Crystal`) false false)
  (`KismetSystemLibrary.Delay` 0.2)
  (`self.FinishActivate` anInstigator))

(event `self.OnEnable`
  (bind _ns_crystal (`self.NS_Crystal`))
  (`SceneComponent.SetVisibility` _ns_crystal true false)
  (`ActorComponent.Activate` _ns_crystal false)
  (`SceneComponent.SetVisibility` (`self.PointLight`) true false))

(fn `UserConstructionScript`)