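; BP_ArrowProjectile is a projectile actor for the arrow obstacle that destroys itself after its Lifetime expires.
; Each Tick it runs a multi sphere trace along its next step, ignoring its owner and drawing debug shapes, then moves by Velocity without sweeping.
; Movement is per frame with no delta-time scaling, and the trace results are not used, so hits have no effect.
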(event `self.ReceiveBeginPlay`
  (`KismetSystemLibrary.Delay` (`self.Lifetime`))
  (`self.K2_DestroyActor`))

(event `self.ReceiveTick`
  (params (DeltaSeconds :type "Float (single-precision)"))
  (bind _returnvalue (`self.K2_GetActorLocation`))
  (`KismetSystemLibrary.SphereTraceMulti` _returnvalue (+ _returnvalue (`self.Velocity`)) (`self.Radius`) "TraceTypeQuery1" false (`|MakeArray` (`self.GetOwner`)) "ForDuration" true (struct :`R` 1.0 :`A` 1.0) (struct :`G` 1.0 :`A` 1.0) 0.1)
  (`self.K2_SetActorLocation` (+ (`self.K2_GetActorLocation`) (`self.Velocity`))))

(fn `UserConstructionScript`)