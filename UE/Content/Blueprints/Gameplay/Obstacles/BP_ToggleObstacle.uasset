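; BP_ToggleObstacle is an obstacle that cycles endlessly between active and inactive states on a timer.
; On BeginPlay it disables itself and waits a random time up to StartDuration before starting the cycle.
; The Update event calls Enable, waits ActiveDuration, calls Disable, waits InactiveDuration, then calls itself again.
; Enable and Disable are empty here, so the asset supplies only the timing.
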(event `self.ReceiveBeginPlay`
  (`self.Disable`)
  (`KismetSystemLibrary.Delay` (`KismetMathLibrary.RandomFloatInRange` 0.0 (`self.StartDuration`)))
  (`self.Update`))

(event `Update`
  (`self.Enable`)
  (`KismetSystemLibrary.Delay` (`self.ActiveDuration`))
  (`self.Disable`)
  (`KismetSystemLibrary.Delay` (`self.InactiveDuration`))
  (`self.Update`))

(fn `Disable`)

(fn `Enable`)

(fn `UserConstructionScript`)