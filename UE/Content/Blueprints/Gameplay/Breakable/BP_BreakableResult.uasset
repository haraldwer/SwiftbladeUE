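; Debris actor for breakables that turns supplied mesh components into short-lived physics pieces.
; BreakMeshes either copies each mesh whole or slices it along a plane into two capped procedural halves.
; Halves ride on generated box or sphere colliders instead of their own collision; all pieces block only WorldStatic and get random impulses.
; After Lifetime, a throttled Tick shrinks the pieces, then destroys the actor.
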(event `self.ReceiveBeginPlay`
  (`self.SetActorTickInterval` 0.1)
  (`self.SetActorTickEnabled` false)
  (`KismetSystemLibrary.Delay` (`self.Lifetime`))
  (`self.SetActorTickEnabled` true))

(event `self.ReceiveTick`
  (params (DeltaSeconds :type "Float (single-precision)"))
  (bind _output_get (set `self.Scale` (- (`self.Scale`) (* DeltaSeconds 2.0))))
  (if (> _output_get 0.0)
    (for _array_element (`self.Meshes`)
      (`SceneComponent.SetRelativeScale3D` _array_element (`KismetMathLibrary.Conv_DoubleToVector` _output_get)))
    (else
      (`self.K2_DestroyActor`))))

(event `self.BreakMeshes`
  (params (someComponents :type "Array of StaticMeshComponent Object Reference (by ref)") (aPosition :type "Vector Structure (by ref)") (aNormal :type "Vector Structure (by ref)") (aSplit :type Boolean))
  (for _array_element someComponents
    (`self.BreakMesh` _array_element aPosition aNormal aSplit)))

(event `self.ReceiveHit`
  (params (MyComp :type "PrimitiveComponent Object Reference") (Other :type "Actor Object Reference") (OtherComp :type "PrimitiveComponent Object Reference") (bSelfMoved :type Boolean) (HitLocation :type "Vector Structure") (HitNormal :type "Vector Structure") (NormalImpulse :type "Vector Structure") (Hit :type "HitResult Structure (by ref)"))
  (`KismetSystemLibrary.PrintString` (`KismetSystemLibrary.GetDisplayName` MyComp))
  (`KismetSystemLibrary.PrintString` (`KismetSystemLibrary.GetDisplayName` OtherComp)))

(fn `BreakMesh`
  (params (Mesh :type "StaticMeshComponent Object Reference") (Position :type "Vector Structure") (Normal :type "Vector Structure") (Split :type Boolean))
  (`/Engine/EditorBlueprintResources/StandardMacros.IsValid` Mesh
    (:`Is Valid`
      (if Split
        (bind _returnvalue (`|AddComponentByClass` "/Script/ProceduralMeshComponent.ProceduralMeshComponent"))
        (`self.SetupProcMeshComp` Mesh _returnvalue)
        (`KismetProceduralMeshLibrary.CopyProceduralMeshFromStaticMeshComponent` Mesh 0 _returnvalue true)
        (bind _outotherhalfprocmesh (`KismetProceduralMeshLibrary.SliceProceduralMesh` _returnvalue Position Normal true "CreateNewSectionForCap" (`self.CapMaterial`)))
        (`self.SetupProcMeshComp` Mesh _outotherhalfprocmesh)
        (else
          (bind _returnvalue_2 (`self.CreateStatMesh`))
          (`StaticMeshComponent.SetStaticMesh` _returnvalue_2 (`StaticMeshComponent.StaticMesh` Mesh))
          (`SceneComponent.K2_AttachToComponent` _returnvalue_2 (`self.DefaultSceneRoot`) "None" "KeepRelative" "KeepRelative" "KeepRelative" true)
          (`SceneComponent.K2_SetWorldTransform` _returnvalue_2 (`SceneComponent.K2_GetComponentToWorld` Mesh) false false)
          (`self.SetupRendering` Mesh _returnvalue_2)
          (`self.SetupCollisions` _returnvalue_2)
          (`self.SetupPhysics` _returnvalue_2))))))

(fn `CreateProcMesh`
  (returns (ReturnValue :type "ProceduralMeshComponent Object Reference"))
  (bind _returnvalue (`|AddComponentByClass` "/Script/ProceduralMeshComponent.ProceduralMeshComponent"))
  (`KismetArrayLibrary.Array_Add` (`self.Meshes`) _returnvalue)
  (return _returnvalue))

(fn `CreateStatMesh`
  (returns (ReturnValue :type "StaticMeshComponent Object Reference"))
  (bind _returnvalue (`|AddComponentByClass` "/Script/Engine.StaticMeshComponent"))
  (`KismetArrayLibrary.Array_Add` (`self.Meshes`) _returnvalue)
  (return _returnvalue))

(fn `GenerateSimpleCollider`
  (params (Component :type "ProceduralMeshComponent Object Reference"))
  (returns (NewParam :type "ShapeComponent Object Reference"))
  (locals (Verts :type "Array of Vector Structure"))
  (bind (_origin _boxextent) (`KismetSystemLibrary.GetComponentBounds` Component))
  (bind (_origin_2 _boxextent_2 _sphereradius) (`KismetSystemLibrary.GetComponentBounds` Component))
  (if (`self.UseBox`)
    (`ProceduralMeshComponent.ClearCollisionConvexMeshes` Component)
    (bind _returnvalue (`|AddComponentByClass` "/Script/Engine.BoxComponent"))
    (`BoxComponent.SetBoxExtent` _returnvalue _boxextent true)
    (`SceneComponent.K2_SetWorldLocation` _returnvalue _origin false false)
    (`SceneComponent.K2_AttachToComponent` Component _returnvalue "None" "KeepWorld" "KeepRelative" "KeepWorld" true)
    (return _returnvalue)
    (else
      (`ProceduralMeshComponent.ClearCollisionConvexMeshes` Component)
      (bind _returnvalue_2 (`|AddComponentByClass` "/Script/Engine.SphereComponent"))
      (`SphereComponent.SetSphereRadius` _returnvalue_2 _sphereradius true)
      (`SceneComponent.K2_SetWorldLocation` _returnvalue_2 _origin_2 false false)
      (`SceneComponent.K2_AttachToComponent` Component _returnvalue_2 "None" "KeepWorld" "KeepRelative" "KeepWorld" true)
      (return _returnvalue_2))))

(fn `SetupCollisions`
  (params (Shape :type "PrimitiveComponent Object Reference"))
  (`PrimitiveComponent.SetCollisionResponseToAllChannels` Shape "ECR_Ignore")
  (`PrimitiveComponent.SetCollisionResponseToChannel` Shape "ECC_WorldStatic" "ECR_Block")
  (`PrimitiveComponent.SetCollisionObjectType` Shape "ECC_Destructible")
  (`PrimitiveComponent.SetCollisionEnabled` Shape "QueryAndPhysics"))

(fn `SetupPhysics`
  (params (Shape :type "PrimitiveComponent Object Reference"))
  (`PrimitiveComponent.SetPhysicsMaxAngularVelocityInDegrees` Shape 50.0 false "None")
  (`PrimitiveComponent.SetAngularDamping` Shape 0.5)
  (`PrimitiveComponent.SetLinearDamping` Shape 0.2)
  (`PrimitiveComponent.SetSimulatePhysics` Shape true)
  (`PrimitiveComponent.AddImpulse` Shape (* (`KismetMathLibrary.RandomUnitVector`) (`self.ImpulseStrength`)) "None" true))

(fn `SetupProcMeshComp`
  (params (StaticMesh :type "StaticMeshComponent Object Reference") (Result :type "ProceduralMeshComponent Object Reference"))
  (`SceneComponent.K2_AttachToComponent` Result (`self.DefaultSceneRoot`) "None" "KeepRelative" "KeepRelative" "KeepRelative" false)
  (`KismetArrayLibrary.Array_Add` (`self.Meshes`) Result)
  (`SceneComponent.K2_SetWorldTransform` Result (`SceneComponent.K2_GetComponentToWorld` StaticMesh) false false)
  (`self.SetupRendering` StaticMesh Result)
  (`PrimitiveComponent.SetCollisionEnabled` Result "NoCollision")
  (bind _newparam (`self.GenerateSimpleCollider` Result))
  (`self.SetupCollisions` _newparam)
  (`self.SetupPhysics` _newparam))

(fn `SetupRendering`
  (params (StaticMesh :type "StaticMeshComponent Object Reference") (Result :type "PrimitiveComponent Object Reference"))
  (`SceneComponent.SetVisibility` Result (`SceneComponent.bVisible` StaticMesh) false)
  (`SceneComponent.SetHiddenInGame` Result (`SceneComponent.bHiddenInGame` StaticMesh) false)
  (`PrimitiveComponent.SetMaterial` Result 0 (`PrimitiveComponent.GetMaterial` StaticMesh 0))
  (return))

(fn `UserConstructionScript`)