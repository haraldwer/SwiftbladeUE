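; First-person player controller that forwards left mouse clicks to the character's widget interaction and handles saving and loading state.
; Press sends a pointer key, while release calls ReleaseKey rather than ReleasePointerKey.
; SaveState writes the current state through BP_SaveObject to a single default slot.
; LoadState acts only in the Base level, restoring that slot, except that non-distribution builds skip it on the game instance's first load.
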(event `Key|LeftMouseButton` :consume false
  (params (Key :type "Key Structure"))
  (bind _returnvalue (`self.GetFPCharacter`))
  (:`Pressed`
    (bind _asbp_fpcharacter (cast `/Game/Blueprints/Player/BP_FPCharacter` _returnvalue))
    (`/Engine/EditorBlueprintResources/StandardMacros.IsValid` _returnvalue
      (:`Is Valid`
        (`WidgetInteractionComponent.PressPointerKey` (`/Game/Blueprints/Player/BP_FPCharacter.WidgetInteraction` _asbp_fpcharacter) Key))))
  (:`Released`
    (bind _asbp_fpcharacter_2 (cast `/Game/Blueprints/Player/BP_FPCharacter` _returnvalue))
    (`/Engine/EditorBlueprintResources/StandardMacros.IsValid` _returnvalue
      (:`Is Valid`
        (`WidgetInteractionComponent.ReleaseKey` (`/Game/Blueprints/Player/BP_FPCharacter.WidgetInteraction` _asbp_fpcharacter_2) Key)))))

(event `self.SaveState`
  (bind _returnvalue (`GameplayStatics.CreateSaveGameObject` "/Game/Blueprints/Player/BP_SaveObject.BP_SaveObject_C"))
  (`/Game/Blueprints/Player/BP_SaveObject.SetFromState` _returnvalue (`self.GetState`))
  (`GameplayStatics.SaveGameToSlot` _returnvalue "DefaultSave"))

(event `self.LoadState`
  (bind _returnvalue (`GameplayStatics.GetCurrentLevelName` true))
  (if (`KismetStringLibrary.EqualEqual_StrStr` _returnvalue "Base")
    (if (`KismetSystemLibrary.IsPackagedForDistribution`)
      (bind _returnvalue_2 (`GameplayStatics.LoadGameFromSlot` "DefaultSave" :!label _label))
      (bind _asbp_save_object (cast `/Game/Blueprints/Player/BP_SaveObject` _returnvalue_2)
        (:`then`
          (`self.OnStateLoaded` (`/Game/Blueprints/Player/BP_SaveObject.Get State` _asbp_save_object)))
        (:`CastFailed`
          (`self.OnStateLoaded` (struct) :!label _label_2)))
      (else
        (bind _asbp_game_instance (cast `/Game/Blueprints/BP_GameInstance` (`GameplayStatics.GetGameInstance`))
          (:`then`
            (if (`/Game/Blueprints/BP_GameInstance.FirstStateLoad` _asbp_game_instance)
              (set `/Game/Blueprints/BP_GameInstance.FirstStateLoad` false _asbp_game_instance)
              (goto _label_2)
              (else
                (goto _label))))
          (:`CastFailed`
            (goto _label_2)))))))

(fn `UserConstructionScript`)