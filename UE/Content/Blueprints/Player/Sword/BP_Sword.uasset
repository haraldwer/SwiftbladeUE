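; Player sword actor that drives two visual effects every tick: surface-contact particles and a blade trail.
; A visibility line trace along the blade toggles the intersect Niagara spawn rate and moves that effect to just short of the hit point.
; The trail mesh's X scale follows the Strength scalar from the Params_Magic material parameter collection.
; An older velocity-based trail scale and emitter toggling remain unconnected.
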(event `self.ReceiveTick`
  (params (DeltaSeconds :type "Float (single-precision)"))
  (`self.IntersectEffect`)
  (`self.ScaleTrailMesh`))

(fn `IntersectEffect`
  (bind _returnvalue (`self.GetTransform`))
  (bind _ns_swordintersect (`self.NS_SwordIntersect`))
  (bind (_outhit _returnvalue_2) (`KismetSystemLibrary.LineTraceSingle` (`KismetMathLibrary.TransformLocation` _returnvalue (0.0 0.0 15.0)) (`KismetMathLibrary.TransformLocation` _returnvalue (0.0 0.0 100.0)) "TraceTypeQuery1"))
  (`FXSystemComponent.SetFloatParameter` _ns_swordintersect "B_SpawnRate" (`KismetMathLibrary.Conv_BoolToDouble` _returnvalue_2))
  (if _returnvalue_2
    (`SceneComponent.K2_SetWorldLocation` _ns_swordintersect (- (`.Location` (`GameplayStatics.BreakHitResult` _outhit)) (* (`self.GetActorUpVector`) (5.0 5.0 5.0))) false false)))

(fn `ScaleTrailMesh`
  (bind _returnvalue (`KismetMaterialLibrary.GetScalarParameterValue` "/Game/Blueprints/Player/PostProcessing/Params_Magic.Params_Magic" "Strength"))
  (`SceneComponent.SetRelativeScale3D` (`self.SwordTrail`) (`KismetMathLibrary.MakeVector` _returnvalue 1.0 1.0)))

(fn `UserConstructionScript`)