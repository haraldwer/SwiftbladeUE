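; BP_Enemy is a physics-driven enemy that chases the player once the player comes within range.
; Each tick, while the player is closer than MinDist to the Cube, it stores the player's location as the target and latches HasTarget.
; It then smoothly rotates the Cube toward that target and pushes it forward with mass-independent force, heading for the last seen position if the player leaves range.
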(event `self.ReceiveTick`
  (params (DeltaSeconds :type "Float (single-precision)"))
  (bind _returnvalue (`self.K2_GetActorLocation` (`GameplayStatics.GetPlayerPawn` 0)))
  (`|ExecutionSequence`
    (:`then_0`
      (if (< (`KismetMathLibrary.Vector_Distance` _returnvalue (`SceneComponent.K2_GetComponentLocation` (`self.Cube`))) (`self.MinDist`))
        (set `self.TargetPosition` _returnvalue)
        (set `self.HasTarget` true)))
    (:`then_1`
      (if (`self.HasTarget`)
        (`SceneComponent.K2_SetWorldRotation` (`self.Cube`) (`KismetMathLibrary.RInterpTo` (`SceneComponent.K2_GetComponentRotation` (`self.Cube`)) (`KismetMathLibrary.FindLookAtRotation` (`SceneComponent.K2_GetComponentLocation` (`self.Cube`)) (`self.TargetPosition`)) DeltaSeconds (`self.RotationSpeed`)) false false)
        (`PrimitiveComponent.AddForce` (`self.Cube`) (* (`SceneComponent.GetForwardVector` (`self.Cube`)) (`self.ForwardForce`)) "None" true)))))

(fn `UserConstructionScript`)