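; BP_ProceduralPlatform is a platform actor that builds a flat-topped procedural mesh from a static mesh.
; Its Construction Script copies the StaticMesh component into the ProceduralMesh component with collision enabled.
; It then slices that mesh with a downward-facing horizontal plane at CapHeight above the actor's location, keeping the part below.
; The cut is capped as a new mesh section using CapMaterial.
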(fn `UserConstructionScript`
  (`KismetProceduralMeshLibrary.CopyProceduralMeshFromStaticMeshComponent` (`self.StaticMesh`) 0 (`self.ProceduralMesh`) true)
  (`KismetProceduralMeshLibrary.SliceProceduralMesh` (`self.ProceduralMesh`) (+ (`KismetMathLibrary.MakeVector` 0.0 0.0 (`self.CapHeight`)) (`self.K2_GetActorLocation`)) (`KismetMathLibrary.Vector_Down`) false "CreateNewSectionForCap" (`self.CapMaterial`)))