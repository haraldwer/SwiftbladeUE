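; Procedural stairs actor that lays mesh instances as steps along a spline, built in the construction script through DefaultConstruct.
; StepSpline adds a random mesh at the midpoint of each StepLength segment, scaled to BlockSize with mesh-size compensation, then returns the advanced distance.
; Each step follows the spline's position but keeps only its yaw, staying level on slopes, with a random flip rotation for variety.
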(fn `StepSpline`
  (params (CurrentLength :type "Float (double-precision)") (TargetLength :type "Float (double-precision)"))
  (returns (ResultingLength :type "Float (double-precision)"))
  (locals (Mesh :type "StaticMesh Object Reference"))
  (set `local.Mesh` (`self.GetRandomMesh`))
  (`self.AddInstance` (`local.Mesh`) (`KismetMathLibrary.MakeTransform` (.location (`SplineComponent.GetTransformAtDistanceAlongSpline` (`self.Spline`) (+ (`local.CurrentLength`) (* (`self.StepLength`) 0.5)) "Local" false)) (`KismetMathLibrary.ComposeRotators` (`self.GetRandomFlipRotator`) (`KismetMathLibrary.MakeRotator` 0.0 0.0 (.yaw (.rotation (`SplineComponent.GetTransformAtDistanceAlongSpline` (`self.Spline`) (+ (`local.CurrentLength`) (* (`self.StepLength`) 0.5)) "Local" false))))) (`self.AdjustScaleForMeshSize` (`local.Mesh`) (* (.scale (`SplineComponent.GetTransformAtDistanceAlongSpline` (`self.Spline`) (+ (`local.CurrentLength`) (* (`self.StepLength`) 0.5)) "Local" false)) (`self.BlockSize`)))))
  (return (+ (`local.CurrentLength`) (`self.StepLength`))))

(fn `UserConstructionScript`
  (`self.DefaultConstruct`))