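; BP_ProceduralSpline is a level-building Blueprint that fills a spline with instanced copies of a static mesh in the Construction Script.
; It steps along the spline by StepSize until the end or MaxIterations, placing each instance at the segment midpoint, aimed at the next point.
; Roll accumulates a quarter turn plus random jitter per piece, using a fixed-seed stream so the layout rebuilds identically.
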(fn `UserConstructionScript`
  (locals (Iterations :type Integer) (TargetLength :type "Float (double-precision)") (Length :type "Float (double-precision)") (NextLength :type "Float (double-precision)") (Rotation :type "Float (double-precision)"))
  (bind _randomrotation (`self.RandomRotation`))
  (bind _spline (`self.Spline`))
  (bind _returnvalue (`SplineComponent.GetLocationAtDistanceAlongSpline` _spline (`local.NextLength`) "Local"))
  (bind _returnvalue_2 (`SplineComponent.GetLocationAtDistanceAlongSpline` _spline (`local.Length`) "Local"))
  (`KismetMathLibrary.SetRandomStreamSeed` (`self.Stream`))
  (set `local.Iterations` 0)
  (set `local.Length` 0.0)
  (set `local.TargetLength` (`SplineComponent.GetSplineLength` (`self.Spline`)))
  (while (and (< (`local.Iterations`) (`self.MaxIterations`)) (< (`local.Length`) (`local.TargetLength`)))
    (set `local.Iterations` (+ (`local.Iterations`) 1))
    (set `local.NextLength` (+ (`local.Length`) (`self.StepSize`)))
    (set `local.Rotation` (+ (`local.Rotation`) (+ (`KismetMathLibrary.RandomFloatInRangeFromStream` (* _randomrotation -1.0) _randomrotation (`self.Stream`)) 90.0)))
    (bind _component (`self.GetMeshComponent` (`self.Static Mesh`) (`self.Spline`)))
    (`/Engine/EditorBlueprintResources/StandardMacros.IsValid` _component
      (:`Is Valid`
        (`InstancedStaticMeshComponent.AddInstance` _component (`KismetMathLibrary.MakeTransform` (* (+ _returnvalue_2 _returnvalue) (`KismetMathLibrary.Conv_DoubleToVector` 0.5)) (`KismetMathLibrary.ComposeRotators` (`KismetMathLibrary.MakeRotator` (`local.Rotation`)) (`KismetMathLibrary.FindLookAtRotation` _returnvalue_2 _returnvalue)) (`self.Scale`)) false)
        (set `local.Length` (`local.NextLength`))))))