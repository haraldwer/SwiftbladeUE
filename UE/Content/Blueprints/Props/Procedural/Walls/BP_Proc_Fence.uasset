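; BP_Proc_Fence is a procedural fence prop that builds posts and diagonal rails along a spline from instanced meshes.
; Each StepSpline call places a randomly chosen, randomly flipped vertical post, then advances by StepSize.
; While the next step stays within the spline, it adds a flipped diagonal stick aimed and stretched between height fractions of the current and next posts.
; Mesh scales are adjusted for mesh size to match configured stick dimensions.
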(fn `StepSpline`
  (params (CurrentLength :type "Float (double-precision)") (TargetLength :type "Float (double-precision)"))
  (returns (ResultingLength :type "Float (double-precision)"))
  (locals (NextLength :type "Float (double-precision)") (CurrentMesh :type "StaticMesh Object Reference") (CurrentTransform :type "Transform Structure") (NextTransform :type "Transform Structure") (Start :type "Vector Structure" :default (0.0 0.0 0.0)) (End :type "Vector Structure" :default (0.0 0.0 0.0)))
  (bind (_x _y _z) (`KismetMathLibrary.BreakVector3f` (`self.DiagonalStickSize`)))
  (set `local.NextLength` (+ (`local.CurrentLength`) (`self.StepSize`)))
  (set `local.CurrentTransform` (`SplineComponent.GetTransformAtDistanceAlongSpline` (`self.Spline`) (`local.CurrentLength`) "Local" false))
  (bind _output_get (set `local.CurrentMesh` (`self.GetRandomMesh`)))
  (`self.AddInstance` _output_get (`KismetMathLibrary.ComposeTransforms` (`KismetMathLibrary.MakeTransform` (`KismetMathLibrary.MakeVector` 0.0 0.0 (* (`KismetMathLibrary.BreakVector3f` (`self.VerticalStickSize`)) 0.5)) (`KismetMathLibrary.ComposeRotators` (`self.GetRandomFlipRotator`) (struct :`Pitch` 90.0)) (`self.AdjustScaleForMeshSize` (`local.CurrentMesh`) (`self.VerticalStickSize`))) (`local.CurrentTransform`)))
  (if (< (`local.NextLength`) (`SplineComponent.GetSplineLength` (`self.Spline`)))
    (set `local.NextTransform` (`SplineComponent.GetTransformAtDistanceAlongSpline` (`self.Spline`) (`local.NextLength`) "Local" false))
    (`|ExecutionSequence`
      (:`then_0`
        (set `local.Start` (.location (`KismetMathLibrary.ComposeTransforms` (`KismetMathLibrary.MakeTransform` (`KismetMathLibrary.MakeVector` 0.0 0.0 (* (`KismetMathLibrary.BreakVector3f` (`self.VerticalStickSize`)) (`self.DiagonalStartPart`)))) (`local.CurrentTransform`)))))
      (:`then_1`
        (set `local.End` (.location (`KismetMathLibrary.ComposeTransforms` (`KismetMathLibrary.MakeTransform` (`KismetMathLibrary.MakeVector` 0.0 0.0 (* (`KismetMathLibrary.BreakVector3f` (`self.VerticalStickSize`)) (`self.DiagonalEndPart`)))) (`local.NextTransform`)))))
      (:`then_2`
        (bind _output_get_2 (set `local.CurrentMesh` (`self.DiagonalMesh`)))
        (`self.AddInstance` _output_get_2 (`KismetMathLibrary.MakeTransform` (+ (`KismetMathLibrary.MakeVector` 0.0 (`self.DiagonalOffset`)) (* (+ (`local.Start`) (`local.End`)) (0.5 0.5 0.5))) (`KismetMathLibrary.ComposeRotators` (`self.GetRandomFlipRotator`) (`KismetMathLibrary.FindLookAtRotation` (`local.Start`) (`local.End`))) (`self.AdjustScaleForMeshSize` (`local.CurrentMesh`) (`KismetMathLibrary.MakeVector` (+ (`KismetMathLibrary.Vector_Distance` (`local.Start`) (`local.End`)) _x) _y _z)))))
      (:`then_3`
        (return (`local.NextLength`))))
    (else
      (return (`local.NextLength`)))))

(fn `UserConstructionScript`
  (`self.DefaultConstruct`))