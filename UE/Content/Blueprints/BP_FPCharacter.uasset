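; BP_FPCharacter is a character Blueprint, named as first-person, that drives a speed-line effect from its movement speed.
; Each Tick, it divides the last update velocity's length by max walk speed, clamps the ratio, and smooths it with FInterpTo.
; The squared result is written to the Speed scalar in the Params_SpeedLines material parameter collection, weakening the response at low speeds.
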(event `self.ReceiveTick`
  (params (DeltaSeconds :type "Float (single-precision)"))
  (`self.Update Speed Line Params`))

(fn `Update Speed Line Params`
  (bind _charactermovement (`self.CharacterMovement`))
  (bind _output_get (set `self.SpeedParamSmoothing` (`KismetMathLibrary.FInterpTo` (`self.SpeedParamSmoothing`) (`KismetMathLibrary.FClamp` (/ (`KismetMathLibrary.VSize` (`CharacterMovementComponent.GetLastUpdateVelocity` _charactermovement)) (`CharacterMovementComponent.MaxWalkSpeed` _charactermovement)) 0.0 1.5) (`GameplayStatics.GetWorldDeltaSeconds`) 2.0)))
  (`KismetMaterialLibrary.SetScalarParameterValue` "/Game/Effects/Fullscreen/Params_SpeedLines.Params_SpeedLines" "Speed" (`KismetMathLibrary.Square` _output_get)))

(fn `UserConstructionScript`)