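; Procedural wall that builds a rock or block wall from instanced meshes in its construction script.
; Stacks randomly sized rows along a path spline, following a vertical spline for height and profile, with seeded rotation and mesh variation.
; Random holes and optional Perlin-noise destruction break up the body and ragged upper outline.
; Optional top, bottom and end-edge passes add trim before overlapping instances are removed.
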(fn `Generate`
  (locals (RowLength :type "Float (double-precision)") (RockLength :type "Float (double-precision)") (Iterations :type Integer) (HeightOffset :type "Float (double-precision)") (TargetLength :type "Float (double-precision)") (EdgeSplineTrans :type "Transform Structure") (EdgeIsFirst :type Boolean) (EdgeTempTrans :type "Transform Structure") (EdgeTempForward :type "Vector Structure") (CurrentRowHeight :type "Float (double-precision)") (CurrentTopRowMeshSize :type "Vector Structure"))
  (bind _verticalspline (`self.VerticalSpline`))
  (bind _heightoffset (`local.HeightOffset`))
  (bind _spline (`self.Spline`))
  (bind _returnvalue (`SplineComponent.GetSplineLength` (`self.VerticalSpline`)))
  (bind (_min _max) (break `Box` (`StaticMesh.GetBoundingBox` (`self.EdgeMesh`))))
  (`self.ClearMeshComponents`)
  (`|ExecutionSequence`
    (:`then_0`
      (set `local.TargetLength` (`SplineComponent.GetSplineLength` (`self.Spline`)))
      (set `local.HeightOffset` 0.0)
      (while (< _heightoffset _returnvalue)
        (bind _output_get (set `local.CurrentRowHeight` (`KismetMathLibrary.FMax` (`KismetMathLibrary.FMin` (- _returnvalue _heightoffset) (`KismetMathLibrary.RandomFloatInRangeFromStream` (.z (`self.MeshMinSize`)) (.z (`self.MeshMaxSize`)) (`self.Stream`))) 10.0)))
        (bind _returnvalue_2 (* _output_get 0.5))
        (set `local.HeightOffset` (+ _returnvalue_2 (`local.HeightOffset`)))
        (`KismetMathLibrary.SetRandomStreamSeed` (`self.Stream`) (* (`KismetMathLibrary.Conv_Int64ToInt` (`KismetMathLibrary.Conv_DoubleToInt64` (`local.HeightOffset`))) 1000))
        (set `local.RowLength` 0.0)
        (while (and (< (`local.RowLength`) (`local.TargetLength`)) (< (`local.Iterations`) (`self.MaxIterations`)))
          (set `local.Iterations` (+ (`local.Iterations`) 1))
          (bind _output_get_2 (set `local.RockLength` (`KismetMathLibrary.FMin` (- (`local.TargetLength`) (`local.RowLength`)) (`KismetMathLibrary.RandomFloatInRangeFromStream` (.x (`self.MeshMinSize`)) (.x (`self.MeshMaxSize`)) (`self.Stream`)))))
          (if (and (> _output_get_2 10.0) (and (> (`KismetMathLibrary.RandomFloatInRangeFromStream` 0.0 100.0 (`self.Stream`)) (`self.HoleChance`)) (or (not (`self.ApplyDestruction`)) (< (`local.HeightOffset`) (`KismetMathLibrary.Lerp` (`self.DestructionVerticalOffset`) (`SplineComponent.GetSplineLength` (`self.VerticalSpline`)) (* (+ (`KismetMathLibrary.PerlinNoise1D` (* (+ (`local.RowLength`) (* (`local.RockLength`) 0.5)) (`self.DestructionNoiseScale`))) 1.0) 0.5))))))
            (`self.CreateRock` (`self.GetRandomMesh`) (`KismetMathLibrary.ComposeTransforms` (`KismetMathLibrary.MakeTransform` (0.0 0.0 0.0) (struct :`Yaw` -90.0 :`Roll` 90.0)) (`KismetMathLibrary.ComposeTransforms` (`KismetMathLibrary.ComposeTransforms` (`SplineComponent.GetTransformAtDistanceAlongSpline` (`self.VerticalSpline`) (`local.HeightOffset`) "Local" false) (`KismetMathLibrary.MakeTransform` (0.0 0.0 0.0) (struct :`Yaw` 90.0))) (`SplineComponent.GetTransformAtDistanceAlongSpline` (`self.Spline`) (+ (`local.RowLength`) (* (`local.RockLength`) 0.5)) "Local" false))) (`KismetMathLibrary.MakeVector` (`local.RockLength`) (`KismetMathLibrary.RandomFloatInRangeFromStream` (.y (`self.MeshMinSize`)) (.y (`self.MeshMaxSize`)) (`self.Stream`)) (`local.CurrentRowHeight`)) (`self.Rotation`) true))
          (set `local.RowLength` (+ (`local.RowLength`) (`local.RockLength`))))
        (set `local.HeightOffset` (+ _returnvalue_2 (`local.HeightOffset`)))))
    (:`then_1`
      (if (`self.TopRow`)
        (`KismetMathLibrary.SetRandomStreamSeed` (`self.Stream`))
        (set `local.Iterations` 0)
        (set `local.RowLength` 0.0)
        (while (and (< (`local.Iterations`) (`self.MaxIterations`)) (< (+ (`local.RowLength`) (`self.TopRowSize`)) (`local.TargetLength`)))
          (set `local.Iterations` (+ (`local.Iterations`) 1))
          (bind _output_get_3 (set `local.CurrentTopRowMeshSize` (`KismetMathLibrary.MakeVector` (`self.TopRowSize`) (.y (`self.Random Vector in Range` (`self.MeshMinSize`) (`self.MeshMaxSize`))) (* (.z (`self.Random Vector in Range` (`self.MeshMinSize`) (`self.MeshMaxSize`))) (`self.TopRowHeightScale`)))))
          (`self.CreateRock` (`self.TopRowMesh`) (`KismetMathLibrary.ComposeTransforms` (`KismetMathLibrary.MakeTransform` (`KismetMathLibrary.MakeVector` (* 0.5 (`.Z` (`KismetMathLibrary.BreakVector3f` (`local.CurrentTopRowMeshSize`))))) (struct :`Yaw` -90.0 :`Roll` 90.0)) (`KismetMathLibrary.ComposeTransforms` (`KismetMathLibrary.ComposeTransforms` (`SplineComponent.GetTransformAtDistanceAlongSpline` _verticalspline (`SplineComponent.GetSplineLength` _verticalspline) "Local" false) (`KismetMathLibrary.MakeTransform` (0.0 0.0 0.0) (struct :`Yaw` 90.0))) (`KismetMathLibrary.MakeTransform` (.location (`SplineComponent.GetTransformAtDistanceAlongSpline` (`self.Spline`) (+ (`local.RowLength`) (* (`self.TopRowSize`) 0.5)) "Local" false)) (.rotation (`SplineComponent.GetTransformAtDistanceAlongSpline` (`self.Spline`) (+ (`local.RowLength`) (* (`self.TopRowSize`) 0.5)) "Local" false)) (.scale (`SplineComponent.GetTransformAtDistanceAlongSpline` (`self.Spline`) (+ (`local.RowLength`) (* (`self.TopRowSize`) 0.5)) "Local" false))))) _output_get_3 (`self.Rotation`) true)
          (set `local.RowLength` (+ (`local.RowLength`) (+ (`self.TopRowSize`) (`self.TopRowSpace`)))))))
    (:`then_2`
      (if (`self.BottomRow`)
        (`KismetMathLibrary.SetRandomStreamSeed` (`self.Stream`))
        (set `local.Iterations` 0)
        (set `local.RowLength` 0.0)
        (while (and (< (`local.Iterations`) (`self.MaxIterations`)) (< (`local.RowLength`) (`local.TargetLength`)))
          (set `local.Iterations` (+ (`local.Iterations`) 1))
          (bind _output_get_4 (set `local.RockLength` (`KismetMathLibrary.FMin` (- (`local.TargetLength`) (`local.RowLength`)) (.x (`self.BottomMeshSize`)))))
          (if (> (`local.RockLength`) 5.0)
            (`self.CreateRock` (`self.BottomRowMesh`) (`KismetMathLibrary.MakeTransform` (+ (.location (`SplineComponent.GetTransformAtDistanceAlongSpline` (`self.Spline`) (+ (`local.RowLength`) (* _output_get_4 0.5)) "Local" false)) (`KismetMathLibrary.MakeVector` 0.0 0.0 (* (.z (`self.BottomMeshSize`)) 0.5))) (.rotation (`SplineComponent.GetTransformAtDistanceAlongSpline` (`self.Spline`) (+ (`local.RowLength`) (* _output_get_4 0.5)) "Local" false)) (.scale (`SplineComponent.GetTransformAtDistanceAlongSpline` (`self.Spline`) (+ (`local.RowLength`) (* _output_get_4 0.5)) "Local" false))) (`KismetMathLibrary.MakeVector` (`local.RockLength`) (.y (`self.BottomMeshSize`)) (.z (`self.BottomMeshSize`))) 0.0 true))
          (set `local.RowLength` (+ (`local.RowLength`) (`local.RockLength`))))))
    (:`then_3`
      (if (`self.Edges`)
        (`KismetMathLibrary.SetRandomStreamSeed` (`self.Stream`) 150)
        (`|ExecutionSequence`
          (:`then_0`
            (set `local.EdgeSplineTrans` (`SplineComponent.GetTransformAtDistanceAlongSpline` _spline 0.0001 "Local" false))
            (set `local.EdgeIsFirst` true))
          (:`then_1`
            (set `local.EdgeSplineTrans` (`SplineComponent.GetTransformAtDistanceAlongSpline` _spline (`SplineComponent.GetSplineLength` _spline) "Local" false))
            (set `local.EdgeIsFirst` false)))
        (set `local.TargetLength` (`SplineComponent.GetSplineLength` (`self.VerticalSpline`)))
        (set `local.Iterations` 0)
        (set `local.RowLength` 0.0)
        (while (and (< (`local.Iterations`) (`self.MaxIterations`)) (< (`local.RowLength`) (`local.TargetLength`)))
          (set `local.Iterations` (+ (`local.Iterations`) 1))
          (`/Engine/EditorBlueprintResources/StandardMacros.IsValid` (`self.EdgeMesh`)
            (:`Is Valid`
              (set `local.RockLength` (`KismetMathLibrary.FMin` (- (`local.TargetLength`) (`local.RowLength`)) (.z (`self.Random Vector in Range` (`self.EdgeMinSize`) (`self.EdgeMaxSize`)))))
              (bind _output_get_5 (set `local.EdgeTempTrans` (`local.EdgeSplineTrans`)))
              (set `local.EdgeTempTrans` (`KismetMathLibrary.ComposeTransforms` (`KismetMathLibrary.MakeTransform` (0.0 0.0 0.0) (struct :`Yaw` -90.0 :`Roll` 90.0)) (`KismetMathLibrary.ComposeTransforms` (`KismetMathLibrary.ComposeTransforms` (`SplineComponent.GetTransformAtDistanceAlongSpline` (`self.VerticalSpline`) (+ (`local.RowLength`) (* (`local.RockLength`) 0.5)) "Local" false) (`KismetMathLibrary.MakeTransform` (0.0 0.0 0.0) (struct :`Yaw` 90.0))) _output_get_5)))
              (bind _output_get_6 (set `local.EdgeTempTrans` (`KismetMathLibrary.MakeTransform` (.location (`local.EdgeTempTrans`)) (.rotation (`local.EdgeTempTrans`)) (/ (`KismetMathLibrary.MakeVector` (.x (`self.Random Vector in Range` (`self.EdgeMinSize`) (`self.EdgeMaxSize`))) (.y (`self.Random Vector in Range` (`self.EdgeMinSize`) (`self.EdgeMaxSize`))) (`local.RockLength`)) (- _max _min)))))
              (`self.AddInstance` (`self.EdgeMesh`) _output_get_6)
              (set `local.RowLength` (+ (`local.RowLength`) (`local.RockLength`))))))))
    (:`then_4`
      (`self.RemoveOverlappingInstances`))))

(fn `GetSpline`
  (params (anIndex :type Integer))
  (returns (ReturnValue :type "SplineComponent Object Reference"))
  (return (select `int` anIndex :`0` (`self.Spline`) :`1` (`self.VerticalSpline`))))

(fn `UserConstructionScript`
  (locals (RowLength :type "Float (double-precision)") (RockLength :type "Float (double-precision)") (Iterations :type Integer) (HeightOffset :type "Float (double-precision)") (TargetLength :type "Float (double-precision)") (EdgeSplineTrans :type "Transform Structure") (EdgeIsFirst :type Boolean) (EdgeTempTrans :type "Transform Structure") (EdgeTempForward :type "Vector Structure") (CurrentRowHeight :type "Float (double-precision)") (CurrentTopRowMeshSize :type "Vector Structure" :default (0.0 0.0 0.0)))
  (`self.Generate`))