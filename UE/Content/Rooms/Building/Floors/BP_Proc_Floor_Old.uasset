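; Procedural floor that fills the area outlined by a spline with randomized instanced mesh tiles, rebuilt in the construction script.
; It computes padded world bounds from the spline points, then walks a tile-sized grid across them, capped by an iteration limit.
; Cells count as inside by a dot product against the nearest spline right vector, so winding direction matters.
; Each tile takes a mesh and quarter-turn yaw from a random stream.
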(fn `UserConstructionScript`
  (locals (TotalLength :type "Float (double-precision)") (MinPos :type "Vector Structure") (MaxPos :type "Vector Structure") (Pos :type "Vector Structure") (Iterations :type Integer) (NextPos :type "Vector Structure"))
  (bind _pos (`local.Pos`))
  (bind _spline (`self.Spline`))
  (bind _returnvalue (`SplineComponent.GetNumberOfSplinePoints` (`self.Spline`)))
  (`self.ClearMeshComponents`)
  (set `local.TotalLength` (`SplineComponent.GetSplineLength` (`self.Spline`)))
  (if (> _returnvalue 0)
    (bind _output_get (set `local.MinPos` (`SplineComponent.GetLocationAtSplinePoint` (`self.Spline`) 0 "World")))
    (set `local.MaxPos` _output_get)
    (for _index (range (+ _returnvalue 1))
      (bind _returnvalue_2 (`SplineComponent.GetLocationAtSplinePoint` (`self.Spline`) _index "World"))
      (set `local.MinPos` (- (`KismetMathLibrary.MakeVector` (`KismetMathLibrary.FMin` (.x _returnvalue_2) (.x (`local.MinPos`))) (`KismetMathLibrary.FMin` (.y _returnvalue_2) (.y (`local.MinPos`))) (`KismetMathLibrary.FMin` (.z _returnvalue_2) (.z (`local.MinPos`)))) (`self.Padding`)))
      (set `local.MaxPos` (+ (`KismetMathLibrary.MakeVector` (`KismetMathLibrary.FMax` (.x _returnvalue_2) (.x (`local.MaxPos`))) (`KismetMathLibrary.FMax` (.y _returnvalue_2) (.y (`local.MaxPos`))) (`KismetMathLibrary.FMax` (.z _returnvalue_2) (.z (`local.MaxPos`)))) (`self.Padding`))))
    (set `local.Iterations` 0)
    (set `local.Pos` (`local.MinPos`))
    (while (and (< (`local.Iterations`) (`self.MaxIterations`)) (< (.y (`local.Pos`)) (.y (`local.MaxPos`))))
      (set `local.Iterations` (+ (`local.Iterations`) 1))
      (if (< (`KismetMathLibrary.Dot_VectorVector` (`SplineComponent.FindRightVectorClosestToWorldLocation` _spline _pos "World") (- (`SplineComponent.FindLocationClosestToWorldLocation` _spline _pos "World") _pos)) 0.0)
        (bind _component (`self.GetMeshComponent` (`KismetArrayLibrary.Array_RandomFromStream` (`self.Meshes`) (`self.Stream`)) (`self.Spline`)))
        (`/Engine/EditorBlueprintResources/StandardMacros.IsValid` _component
          (:`Is Valid`
            (`InstancedStaticMeshComponent.AddInstance` _component (`KismetMathLibrary.MakeTransform` (`local.Pos`) (`KismetMathLibrary.MakeRotator` 0.0 0.0 (+ (* (`KismetMathLibrary.Conv_BoolToDouble` (`KismetMathLibrary.RandomBoolFromStream` (`self.Stream`))) 180.0) (* (`KismetMathLibrary.Conv_BoolToDouble` (`KismetMathLibrary.RandomBoolFromStream` (`self.Stream`))) 90.0))) (`KismetMathLibrary.Conv_DoubleToVector` (`self.TileSize`))) true))))
      (set `local.NextPos` (+ (`local.Pos`) (`KismetMathLibrary.MakeVector` (`self.TileSize`))))
      (set `local.Pos` (select `bool` (> (.x (`local.NextPos`)) (.x (`local.MaxPos`))) :`false` (`local.NextPos`) :`true` (`KismetMathLibrary.MakeVector` (.x (`local.MinPos`)) (+ (`self.TileSize`) (.y (`local.Pos`))) (.z (`local.Pos`))))))))