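; Procedural building piece that places instanced pillar meshes along a spline, regenerated by the construction script.
; Each spline step adds one centred pillar, or a pair offset to either side when Double is set, then advances by StepLength.
; AddPillar picks a random mesh, yaws it in seeded quarter turns, and scales width by Size and height by Height adjusted for mesh size.
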(fn `AddPillar`
  (params (CurrentTrans :type "Transform Structure") (Offset :type "Vector Structure"))
  (locals (CurrentMesh :type "StaticMesh Object Reference"))
  (bind _size (`self.Size`))
  (bind _stream (`self.Stream`))
  (bind _output_get (set `local.CurrentMesh` (`self.GetRandomMesh`)))
  (`self.AddInstance` _output_get (`KismetMathLibrary.ComposeTransforms` (`KismetMathLibrary.MakeTransform` (`local.Offset`) (`KismetMathLibrary.MakeRotator` 0.0 0.0 (+ (* (`KismetMathLibrary.Conv_BoolToDouble` (`KismetMathLibrary.RandomBoolFromStream` _stream)) 180.0) (* (`KismetMathLibrary.Conv_BoolToDouble` (`KismetMathLibrary.RandomBoolFromStream` _stream)) 90.0))) (`KismetMathLibrary.MakeVector` _size _size (.z (`self.AdjustScaleForMeshSize` (`local.CurrentMesh`) (`KismetMathLibrary.Conv_DoubleToVector` (`self.Height`)))))) (`local.CurrentTrans`))))

(fn `StepSpline`
  (params (CurrentLength :type "Float (double-precision)") (TargetLength :type "Float (double-precision)"))
  (returns (ResultingLength :type "Float (double-precision)"))
  (locals (CurrentMesh :type "StaticMesh Object Reference") (CurrentTrans :type "Transform Structure"))
  (bind _returnvalue (`KismetMathLibrary.MakeVector` 0.0 (`self.DoubleDistance`)))
  (set `local.CurrentTrans` (`SplineComponent.GetTransformAtDistanceAlongSpline` (`self.Spline`) (`local.CurrentLength`) "Local" false))
  (if (`self.Double`)
    (`self.AddPillar` (`local.CurrentTrans`) _returnvalue)
    (`self.AddPillar` (`local.CurrentTrans`) (* _returnvalue (-1.0 -1.0 -1.0)))
    (else
      (`self.AddPillar` (`local.CurrentTrans`))))
  (return (+ (`local.CurrentLength`) (`self.StepLength`))))

(fn `UserConstructionScript`
  (`self.Generate`))