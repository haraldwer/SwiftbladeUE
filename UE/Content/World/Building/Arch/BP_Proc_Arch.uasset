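; BP_Proc_Arch is a procedural building piece: a pillar with optional arches on its forward, back, left and right sides.
; The construction script assigns the pillar and forward-arch meshes, then scales the pillar to PillarSize using its mesh bounds.
; For each enabled side, SetupArch shows that arch, scales it to ArchSize, and places it at the pillar's top edge facing outward.
; It briefly switches each arch to Movable for these changes, then back to Static.
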(fn `SetupArch`
  (params (Target :type "SceneComponent Object Reference") (Dir :type "Vector Structure"))
  (bind (_min _max) (break `Box` (`StaticMesh.GetBoundingBox` (`self.ArchMesh`))))
  (`SceneComponent.SetVisibility` Target true false)
  (`SceneComponent.SetMobility` (`local.Target`) "Movable")
  (`SceneComponent.SetRelativeScale3D` (`local.Target`) (/ (`self.ArchSize`) (- _max _min)))
  (`SceneComponent.K2_SetRelativeLocation` (`local.Target`) (`KismetMathLibrary.MakeVector` (* (.x (* (`local.Dir`) (`self.PillarSize`))) 0.5) (* (.y (* (`local.Dir`) (`self.PillarSize`))) 0.5) (.z (* (`local.Dir`) (`self.PillarSize`)))) false false)
  (`SceneComponent.K2_SetRelativeRotation` (`local.Target`) (`KismetMathLibrary.Conv_VectorToRotator` (`KismetMathLibrary.MakeVector` (.x (`local.Dir`)) (.y (`local.Dir`)))) false false)
  (`SceneComponent.SetMobility` (`local.Target`) "Static"))

(fn `UserConstructionScript`
  (bind (_min _max) (break `Box` (`StaticMesh.GetBoundingBox` (`self.PillarMesh`))))
  (`|ExecutionSequence`
    (:`then_0`
      (`StaticMeshComponent.SetStaticMesh` (`self.Pillar`) (`self.PillarMesh`))
      (`StaticMeshComponent.SetStaticMesh` (`self.ArchForward`) (`self.ArchMesh`)))
    (:`then_1`
      (`SceneComponent.SetRelativeScale3D` (`self.Pillar`) (/ (`self.PillarSize`) (- _max _min))))
    (:`then_2`
      (`|ExecutionSequence`
        (:`then_0`
          (if (`self.Forward`)
            (`self.SetupArch` (`self.ArchForward`) (1.0 0.0 1.0))))
        (:`then_1`
          (if (`self.Back`)
            (`self.SetupArch` (`self.ArchBack`) (-1.0 0.0 1.0))))
        (:`then_2`
          (if (`self.Left`)
            (`self.SetupArch` (`self.ArchLeft`) (0.0 -1.0 1.0))))
        (:`then_3`
          (if (`self.Right`)
            (`self.SetupArch` (`self.ArchRight`) (0.0 1.0 1.0))))))))