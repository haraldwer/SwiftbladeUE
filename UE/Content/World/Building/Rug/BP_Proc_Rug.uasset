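; Procedural rug Blueprint that extends its parent's spline-based generation with edge pieces at both ends of the rug.
; After the parent Generate runs, AddEdge spawns a static mesh with the edge material at the spline's start and end, offset outward and mirrored on X for the far end.
; Edges drop roll, register as generated components with static mobility, and the spline is finally scaled up uniformly.
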(fn `AddEdge`
  (params (RelativeTransform :type "Transform Structure"))
  (bind _returnvalue (`AddComponent|NODE_AddStaticMeshComponent-1` :`RelativeTransform` (`KismetMathLibrary.MakeTransform` (.location RelativeTransform) (`KismetMathLibrary.MakeRotator` 0.0 (.pitch (.rotation RelativeTransform)) (.yaw (.rotation RelativeTransform))) (.scale RelativeTransform))))
  (`KismetArrayLibrary.Array_Add` (`self.GeneratedComps`) _returnvalue)
  (`StaticMeshComponent.SetStaticMesh` _returnvalue (`self.Static Mesh`))
  (`PrimitiveComponent.SetCollisionEnabled` _returnvalue (`self.CollisionType`))
  (`PrimitiveComponent.SetCollisionObjectType` _returnvalue "ECC_WorldStatic")
  (`SceneComponent.SetMobility` _returnvalue "Static")
  (`PrimitiveComponent.SetMaterial` _returnvalue 0 (`self.EdgeMaterial`)))

(fn `Generate`
  (bind _spline (`self.Spline`))
  (`parent.Generate`)
  (`self.AddEdge` (`KismetMathLibrary.ComposeTransforms` (`KismetMathLibrary.MakeTransform` (-50.0 0.0 0.0)) (`SplineComponent.GetTransformAtDistanceAlongSpline` (`self.Spline`) 0.0 "Local" false)))
  (`self.AddEdge` (`KismetMathLibrary.ComposeTransforms` (`KismetMathLibrary.MakeTransform` (50.0 0.0 0.0) (struct) (-1.0 1.0 1.0)) (`SplineComponent.GetTransformAtDistanceAlongSpline` _spline (`SplineComponent.GetSplineLength` _spline) "Local" false)))
  (`SceneComponent.SetRelativeScale3D` (`self.Spline`) (3.0 3.0 3.0)))

(fn `UserConstructionScript`
  (`parent.UserConstructionScript`))