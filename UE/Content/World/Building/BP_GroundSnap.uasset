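; BP_GroundSnap is a building Blueprint that snaps its static mesh onto the surface along the actor's up axis.
; The Construction Script runs a Visibility line trace from TraceLength above to TraceLength below the actor, ignoring itself and drawing debug for one frame.
; On a hit, it moves the mesh to the impact location plus ObjectOffset along actor up and zeroes its world rotation, ignoring the surface normal.
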(fn `UserConstructionScript`
  (bind _returnvalue (`self.K2_GetActorLocation`))
  (bind _staticmesh (`self.StaticMesh`))
  (bind _returnvalue_2 (* (`self.GetActorUpVector`) (`self.TraceLength`)))
  (bind (_outhit _returnvalue_3) (`KismetSystemLibrary.LineTraceSingle` (+ _returnvalue _returnvalue_2) (- _returnvalue _returnvalue_2) "TraceTypeQuery1" false (`|MakeArray` self :!type "Actor Object Reference") "ForOneFrame"))
  (if _returnvalue_3
    (`SceneComponent.K2_SetWorldLocation` _staticmesh (+ (`.Location` (`GameplayStatics.BreakHitResult` _outhit)) (* (`self.GetActorUpVector`) (`self.ObjectOffset`))) false false)
    (`SceneComponent.K2_SetWorldRotation` :`self` _staticmesh)))