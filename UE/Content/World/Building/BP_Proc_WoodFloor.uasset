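; Procedural wood floor Blueprint that builds plank-and-rail flooring between two splines at construction time.
; StepSpline places a randomly chosen mesh spanning matching points on both splines, mapped by length ratio, with random offset, flip and size.
; Generate runs the parent generation, then lays offset rail segments along each spline, using one random mesh per rail.
; All pieces are mesh instances, scaled to fit their spans and corrected for mesh size.
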(fn `Generate`
  (`parent.Generate`)
  (`self.GenerateRail` (`self.Spline`))
  (`self.GenerateRail` (`self.Spline1`)))

(fn `GenerateRail`
  (params (InSpline :type "SplineComponent Object Reference"))
  (locals (Iterations :type Integer) (Step :type "Float (double-precision)") (Prev :type "Vector Structure") (Mesh :type "StaticMesh Object Reference") (Curr :type "Vector Structure" :default (0.0 0.0 0.0)))
  (bind _prev (`local.Prev`))
  (bind _curr (`local.Curr`))
  (set `local.Prev` (+ (`self.RailOffset`) (`SplineComponent.GetLocationAtDistanceAlongSpline` (`local.InSpline`) 0.0 "Local")))
  (set `local.Mesh` (`self.GetRandomMesh`))
  (while (and (< (`local.Iterations`) (`self.MaxIterations`)) (< (`local.Step`) (`SplineComponent.GetSplineLength` (`local.InSpline`))))
    (set `local.Iterations` (+ (`local.Iterations`) 1))
    (set `local.Step` (+ (`local.Step`) (`self.RailStep`)))
    (set `local.Curr` (+ (`self.RailOffset`) (`SplineComponent.GetLocationAtDistanceAlongSpline` (`local.InSpline`) (`local.Step`) "Local")))
    (`self.AddInstance` (`local.Mesh`) (`KismetMathLibrary.MakeTransform` (* (+ _prev _curr) (0.5 0.5 0.5)) (`KismetMathLibrary.ComposeRotators` (`self.GetRandomFlipRotator`) (`KismetMathLibrary.FindLookAtRotation` _prev _curr)) (`self.AdjustScaleForMeshSize` (`local.Mesh`) (+ (`KismetMathLibrary.MakeVector` (`KismetMathLibrary.Vector_Distance` _prev _curr)) (`self.RailSize`)))))
    (set `local.Prev` (`local.Curr`)))
  (`SceneComponent.SetMobility` (`local.InSpline`) "Static"))

(fn `StepSpline`
  (params (CurrentLength :type "Float (double-precision)") (TargetLength :type "Float (double-precision)"))
  (returns (ResultingLength :type "Float (double-precision)"))
  (locals (Mesh :type "StaticMesh Object Reference"))
  (bind _outitem (`self.GetRandomMesh`))
  (bind _positionoffset (`self.PositionOffset`))
  (bind _returnvalue (+ (`local.CurrentLength`) (* (`self.StepLength`) 0.5)))
  (bind _location (.location (`SplineComponent.GetTransformAtDistanceAlongSpline` (`self.Spline`) _returnvalue "Local" false)))
  (bind _location_2 (.location (`SplineComponent.GetTransformAtDistanceAlongSpline` (`self.Spline1`) (* (/ _returnvalue (`local.TargetLength`)) (`SplineComponent.GetSplineLength` (`self.Spline1`))) "Local" false)))
  (`/Engine/EditorBlueprintResources/StandardMacros.IsValid` _outitem
    (:`Is Valid`
      (set `local.Mesh` _outitem)
      (`self.AddInstance` (`local.Mesh`) (`KismetMathLibrary.MakeTransform` (+ (`self.Random Vector in Range` _positionoffset (* _positionoffset (-1.0 -1.0 -1.0))) (* (+ _location _location_2) (0.5 0.5 0.5))) (`KismetMathLibrary.ComposeRotators` (`self.GetRandomFlipRotator`) (`KismetMathLibrary.FindLookAtRotation` _location _location_2)) (`self.AdjustScaleForMeshSize` (`local.Mesh`) (+ (`KismetMathLibrary.MakeVector` (`KismetMathLibrary.Vector_Distance` _location _location_2)) (`self.Random Vector in Range` (`self.MinBlockSize`) (`self.MaxBlockSize`))))))
      (return (+ (`local.CurrentLength`) (`self.StepLength`))))
    (:`Is Not Valid`
      (return (+ (`local.CurrentLength`) (`self.StepLength`))))))

(fn `UserConstructionScript`
  (`self.Generate`))