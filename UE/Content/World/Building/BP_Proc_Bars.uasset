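; BP_Proc_Bars is a procedural building piece that builds a grid of bars along a spline, with height set by a second vertical spline.
; The spline step places random-mesh instances as uprights, stretched to the vertical spline's length with seeded random yaw.
; Generate runs from the construction script, calling the parent generation, then stacking BP_Proc_Bar child actors at regular height steps, each copying the main spline's point positions.
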(fn `Generate`
  (`parent.Generate`)
  (`self.VerticalMeshes`))

(fn `GetSpline`
  (params (anIndex :type Integer))
  (returns (ReturnValue :type "SplineComponent Object Reference"))
  (return (select `int` anIndex :`0` (`self.Spline`) :`1` (`self.VerticalSpline`))))

(fn `StepSpline`
  (params (CurrentLength :type "Float (double-precision)") (TargetLength :type "Float (double-precision)"))
  (returns (ResultingLength :type "Float (double-precision)"))
  (locals (CurrentTrans :type "Transform Structure") (CurrentMesh :type "StaticMesh Object Reference"))
  (bind _size (`self.Size`))
  (bind _stream (`self.Stream`))
  (set `local.CurrentTrans` (`SplineComponent.GetTransformAtDistanceAlongSpline` (`self.Spline`) (`local.CurrentLength`) "Local" false))
  (bind _output_get (set `local.CurrentMesh` (`self.GetRandomMesh`)))
  (`self.AddInstance` _output_get (`KismetMathLibrary.ComposeTransforms` (`KismetMathLibrary.MakeTransform` (`KismetMathLibrary.MakeVector` 0.0 5.0 (* (`SplineComponent.GetSplineLength` (`self.VerticalSpline`)) 0.5)) (`KismetMathLibrary.MakeRotator` 0.0 0.0 (+ (* (`KismetMathLibrary.Conv_BoolToDouble` (`KismetMathLibrary.RandomBoolFromStream` _stream)) 180.0) (* (`KismetMathLibrary.Conv_BoolToDouble` (`KismetMathLibrary.RandomBoolFromStream` _stream)) 90.0))) (`KismetMathLibrary.MakeVector` _size _size (.z (`self.AdjustScaleForMeshSize` (`local.CurrentMesh`) (`KismetMathLibrary.Conv_DoubleToVector` (`SplineComponent.GetSplineLength` (`self.VerticalSpline`))))))) (`local.CurrentTrans`)))
  (return (+ (`local.CurrentLength`) (`self.StepLength`))))

(fn `UserConstructionScript`
  (`self.Generate`))

(fn `VerticalMeshes`
  (locals (Iterations :type Integer) (CurrentHeight :type "Float (double-precision)"))
  (while (and (< (`local.Iterations`) 1000) (< (+ (`local.CurrentHeight`) (* (`self.VerticalStepLength`) 0.5)) (`SplineComponent.GetSplineLength` (`self.VerticalSpline`))))
    (set `local.Iterations` (+ (`local.Iterations`) 1))
    (set `local.CurrentHeight` (+ (`local.CurrentHeight`) (`self.VerticalStepLength`)))
    (bind _returnvalue (`AddComponent|NODE_AddChildActorComponent-1` :`RelativeTransform` (`KismetMathLibrary.MakeTransform` (`KismetMathLibrary.MakeVector` 0.0 0.0 (- (`local.CurrentHeight`) (* (`self.VerticalStepLength`) 0.5))))))
    (`SceneComponent.SetMobility` _returnvalue "Static")
    (`ChildActorComponent.SetChildActorClass` _returnvalue "/Game/World/Building/BP_Proc_Bar.BP_Proc_Bar_C")
    (bind _asbp_proc_bar (cast `/Game/World/Building/BP_Proc_Bar` (`ChildActorComponent.ChildActor` _returnvalue)))
    (bind _spline (`/Game/World/Procedural/BP_SplineMesh.Spline` _asbp_proc_bar))
    (`SplineComponent.ClearSplinePoints` _spline false)
    (for _index (range (`SplineComponent.GetNumberOfSplinePoints` (`self.Spline`)))
      (`SplineComponent.AddSplinePoint` _spline (`SplineComponent.GetLocationAtSplinePoint` (`self.Spline`) _index "Local") "Local" false))
    (`SplineComponent.UpdateSpline` (`/Game/World/Procedural/BP_SplineMesh.Spline` _asbp_proc_bar))
    (`ProcSplineMesh.GenerateMesh` _asbp_proc_bar)))