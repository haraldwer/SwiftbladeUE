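; Procedural base actor that scatters instanced static meshes along a spline, with StepSpline left as a stub for child classes to fill in.
; GenerateMesh resets the seeded random stream, clears mesh components, then calls StepSpline until the spline length or iteration cap is reached.
; Helpers supply seeded random meshes, vectors and flips, and add instances to per-mesh components.
; A final pass removes instances overlapping the bounds of listed box and sphere exclusion actors.
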(event `self.GenerateMesh`
  (`self.Generate`))

(fn `AddInstance`
  (params (Mesh :type "StaticMesh Object Reference") (InstanceTransform :type "Transform Structure (by ref)") (bWorldSpace :type Boolean))
  (bind _component (`self.GetMeshComponent` Mesh (`self.Spline`)))
  (`/Engine/EditorBlueprintResources/StandardMacros.IsValid` _component
    (:`Is Valid`
      (`InstancedStaticMeshComponent.AddInstance` _component InstanceTransform bWorldSpace)
      (return))
    (:`Is Not Valid`
      (return))))

(fn `Generate`
  (locals (TargetLength :type "Float (double-precision)") (Length :type "Float (double-precision)") (Iterations :type Integer))
  (`self.ResetSeed`)
  (`self.ClearMeshComponents`)
  (set `local.TargetLength` (`SplineComponent.GetSplineLength` (`self.Spline`)))
  (set `local.Length` 0.0)
  (set `local.Iterations` 0)
  (while (and (< (`local.Iterations`) (`self.MaxIterations`)) (< (`local.Length`) (`local.TargetLength`)))
    (set `local.Iterations` (+ (`local.Iterations`) 1))
    (bind _resultinglength (`self.StepSpline` (`local.Length`) (`local.TargetLength`)))
    (set `local.Length` _resultinglength))
  (`self.RemoveOverlappingInstances`)
  (return))

(fn `GetRandomFlipRotator`
  (returns (ReturnValue :type "Rotator Structure"))
  (bind _stream (`self.Stream`))
  (return (`KismetMathLibrary.MakeRotator` (* (`KismetMathLibrary.Conv_BoolToDouble` (`KismetMathLibrary.RandomBoolFromStream` _stream)) 180.0) (* (`KismetMathLibrary.Conv_BoolToDouble` (`KismetMathLibrary.RandomBoolFromStream` _stream)) 180.0) (* (`KismetMathLibrary.Conv_BoolToDouble` (`KismetMathLibrary.RandomBoolFromStream` _stream)) 180.0))))

(fn `GetRandomMesh`
  (returns (OutItem :type "StaticMesh Object Reference"))
  (return (`KismetArrayLibrary.Array_RandomFromStream` (`self.Meshes`) (`self.Stream`))))

(fn `GetSpline`
  (params (anIndex :type Integer))
  (returns (ReturnValue :type "SplineComponent Object Reference"))
  (if (== anIndex 0)
    (return (`self.Spline`))
    (else
      (return null))))

(fn `Random Vector in Range`
  (params (Min :type "Vector Structure") (Max :type "Vector Structure"))
  (returns (Out :type "Vector Structure"))
  (bind _stream (`self.Stream`))
  (return (`KismetMathLibrary.MakeVector` (`KismetMathLibrary.RandomFloatInRangeFromStream` (.x Min) (.x Max) _stream) (`KismetMathLibrary.RandomFloatInRangeFromStream` (.y Min) (.y Max) _stream) (`KismetMathLibrary.RandomFloatInRangeFromStream` (.z Min) (.z Max) _stream))))

(fn `RemoveBoxOverlaps`
  (params (Box :type "Box Structure (by ref)"))
  (bind _values (`BlueprintMapLibrary.Map_Values` (`self.ExistingMeshComponents`)))
  (for _array_element _values
    (bind _returnvalue (`InstancedStaticMeshComponent.GetInstancesOverlappingBox` _array_element Box true))
    (if (`KismetArrayLibrary.Array_IsNotEmpty` _returnvalue)
      (`InstancedStaticMeshComponent.RemoveInstances` _array_element _returnvalue)))
  (return))

(fn `RemoveOverlappingInstances`
  (`|ExecutionSequence`
    (:`then_0`
      (for _array_element (`self.BoxOverlaps`)
        (`/Engine/EditorBlueprintResources/StandardMacros.IsValid` _array_element
          (:`Is Valid`
            (bind (_origin _boxextent) (`self.GetActorBounds` _array_element true true))
            (`self.RemoveBoxOverlaps` (`KismetMathLibrary.MakeBox` (- _origin _boxextent) (+ _origin _boxextent)))))))
    (:`then_1`
      (for _array_element_2 (`self.SphereOverlaps`)
        (`/Engine/EditorBlueprintResources/StandardMacros.IsValid` _array_element_2
          (:`Is Valid`
            (bind (_origin_2 _boxextent_2) (`self.GetActorBounds` _array_element_2 true true))
            (`self.RemoveSphereOverlaps` _origin_2 (/ (`KismetMathLibrary.VSize` _boxextent_2) 2.0))))))))

(fn `RemoveSphereOverlaps`
  (params (Center :type "Vector Structure") (Radius :type "Float (double-precision)"))
  (bind _values (`BlueprintMapLibrary.Map_Values` (`self.ExistingMeshComponents`)))
  (for _array_element _values
    (bind _returnvalue (`InstancedStaticMeshComponent.GetInstancesOverlappingSphere` _array_element Center Radius true))
    (if (`KismetArrayLibrary.Array_IsNotEmpty` _returnvalue)
      (`InstancedStaticMeshComponent.RemoveInstances` _array_element _returnvalue)))
  (return))

(fn `ResetSeed`
  (`KismetMathLibrary.SetRandomStreamSeed` (`self.Stream`))
  (return))

(fn `StepSpline`
  (params (CurrentLength :type "Float (double-precision)") (TargetLength :type "Float (double-precision)"))
  (returns (ResultingLength :type "Float (double-precision)"))
  (return 0.0))

(fn `UserConstructionScript`
  (locals (Length :type "Float (double-precision)") (TargetLength :type "Float (double-precision)") (Iterations :type Integer)))