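; BP_Proc_Mesh is a procedural mesh Blueprint that provides instanced static mesh helpers, with an empty Generate function and construction script.
; GetMeshComponent caches one component per mesh in a map, creating each on demand as static, non-ticking and attached, with configured material and collision.
; ClearMeshComponents clears instances and empties the map without destroying components.
; AdjustScaleForMeshSize divides a desired scale by the mesh's bounding box size.
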(fn `AdjustScaleForMeshSize`
  (params (Mesh :type "StaticMesh Object Reference") (Scale :type "Vector Structure"))
  (returns (ReturnValue :type "Vector Structure"))
  (bind (_min _max) (break `Box` (`StaticMesh.GetBoundingBox` Mesh)))
  (`/Engine/EditorBlueprintResources/StandardMacros.IsValid` Mesh
    (:`Is Valid`
      (return (/ Scale (- _max _min))))
    (:`Is Not Valid`
      (return (1.0 1.0 1.0)))))

(fn `ClearMeshComponents`
  (bind _values (`BlueprintMapLibrary.Map_Values` (`self.ExistingMeshComponents`)))
  (for _array_element _values
    (`InstancedStaticMeshComponent.ClearInstances` _array_element))
  (`BlueprintMapLibrary.Map_Clear` (`self.ExistingMeshComponents`)))

(fn `Generate`)

(fn `GetMeshComponent`
  (params (Mesh :type "StaticMesh Object Reference") (Parent :type "SceneComponent Object Reference"))
  (returns (Component :type "InstancedStaticMeshComponent Object Reference"))
  (bind (_value _returnvalue) (`BlueprintMapLibrary.Map_Find` (`self.ExistingMeshComponents`) Mesh))
  (`/Engine/EditorBlueprintResources/StandardMacros.IsValid` Mesh
    (:`Is Valid`
      (if _returnvalue
        (return _value)
        (else
          (bind _returnvalue_2 (`AddComponent|NODE_AddInstancedStaticMeshComponent-0`))
          (`BlueprintMapLibrary.Map_Add` (`self.ExistingMeshComponents`) Mesh _returnvalue_2)
          (`SceneComponent.K2_AttachToComponent` _returnvalue_2 (`local.Parent`) "None" "KeepRelative" "KeepRelative" "KeepRelative" true)
          (`StaticMeshComponent.SetStaticMesh` _returnvalue_2 Mesh)
          (`PrimitiveComponent.SetMaterial` _returnvalue_2 0 (`self.Material`))
          (`SceneComponent.SetMobility` _returnvalue_2 "Static")
          (`ActorComponent.SetComponentTickEnabled` _returnvalue_2 false)
          (`PrimitiveComponent.SetCollisionResponseToAllChannels` _returnvalue_2 (`self.CollisionResponse`))
          (`PrimitiveComponent.SetCollisionObjectType` _returnvalue_2 "ECC_WorldStatic")
          (set `PrimitiveComponent.bGenerateOverlapEvents` (`self.GenerateOverlapEvents`) _returnvalue_2)
          (return _returnvalue_2))))))

(fn `UserConstructionScript`)