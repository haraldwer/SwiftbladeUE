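; Procedural spline actor that scatters randomly chosen instanced meshes along its spline, regenerating from the construction script via Generate.
; StepSpline advances by StepSize times the random X scale, placing each instance at the segment's midpoint, aimed along it.
; Roll accumulates 90 degrees plus seeded jitter per step, with optional random flipping, and the function returns the next distance.
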(fn `StepSpline`
  (params (CurrentLength :type "Float (double-precision)") (TargetLength :type "Float (double-precision)"))
  (returns (ResultingLength :type "Float (double-precision)"))
  (locals (NextLength :type "Float (double-precision)") (Scale :type "Vector Structure"))
  (bind _randomrotation (`self.RandomRotation`))
  (bind _spline (`self.Spline`))
  (bind _returnvalue (`SplineComponent.GetLocationAtDistanceAlongSpline` _spline (`local.NextLength`) "Local"))
  (bind _returnvalue_2 (`SplineComponent.GetLocationAtDistanceAlongSpline` _spline (`local.CurrentLength`) "Local"))
  (set `local.Scale` (`self.Random Vector in Range` (`self.MinScale`) (`self.MaxScale`)))
  (set `local.NextLength` (+ (`local.CurrentLength`) (* (`self.StepSize`) (.x (`local.Scale`)))))
  (set `self.StepRotation` (+ (`self.StepRotation`) (+ (`KismetMathLibrary.RandomFloatInRangeFromStream` (* _randomrotation -1.0) _randomrotation (`self.Stream`)) 90.0)))
  (`self.AddInstance` (`self.GetRandomMesh`) (`KismetMathLibrary.MakeTransform` (* (+ _returnvalue_2 _returnvalue) (`KismetMathLibrary.Conv_DoubleToVector` 0.5)) (`KismetMathLibrary.ComposeRotators` (* (`self.GetRandomFlipRotator`) (`KismetMathLibrary.Conv_BoolToDouble` (`self.RandomFlip`))) (`KismetMathLibrary.ComposeRotators` (`KismetMathLibrary.MakeRotator` (`self.StepRotation`)) (`KismetMathLibrary.FindLookAtRotation` _returnvalue_2 _returnvalue))) (`local.Scale`)))
  (return (`local.NextLength`)))

(fn `UserConstructionScript`
  (locals (NextLength :type "Float (double-precision)") (Rotation :type "Float (double-precision)"))
  (`self.Generate`))