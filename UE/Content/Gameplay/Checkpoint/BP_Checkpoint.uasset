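; Checkpoint actor: a crystal that appears once enabled and, when activated, bursts into a pickup effect before finishing activation.
; While enabled and unstruck, Tick eases in visibility to drive the material parameter collection, Niagara scale, rise between Start and End, and light, while spinning the crystal.
; Activate triggers time dilation and a crystal post-process, then hides the crystal.
; Once struck, Tick brightens the light and writes the crystal's screen position to the collection.
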(event `self.ReceiveBeginPlay`
  (`KismetMaterialLibrary.SetScalarParameterValue` "/Game/Gameplay/Checkpoint/Param_Crystal.Param_Crystal" "Visibility"))

(event `self.ReceiveTick`
  (params (DeltaSeconds :type "Float (single-precision)"))
  (bind _pointlight (`self.PointLight`))
  (if (`self.IsEnabled`)
    (if (`self.Struck`)
      (`LightComponent.SetIntensity` _pointlight (`KismetMathLibrary.FInterpTo` (`LightComponentBase.Intensity` _pointlight) 30.0 (`GameplayStatics.GetWorldDeltaSeconds`) 1.0))
      (bind _returnvalue (`MainSingelton.GetLocalController`))
      (`/Engine/EditorBlueprintResources/StandardMacros.IsValid` _returnvalue
        (:`Is Valid`
          (bind (_x _y) (`KismetMathLibrary.BreakVector2D` (/ (`GameplayStatics.ProjectWorldToScreen` _returnvalue (`SceneComponent.K2_GetComponentLocation` (`self.Crystal`))) (`WidgetLayoutLibrary.GetViewportSize`))))
          (`KismetMaterialLibrary.SetVectorParameterValue` "/Game/Gameplay/Checkpoint/Param_Crystal.Param_Crystal" "ScreenCoord" (`KismetMathLibrary.MakeColor` (`KismetMathLibrary.FClamp` _x) (`KismetMathLibrary.FClamp` _y)))))
      (else
        (bind _output_get (set `self.CrystalVisibility` (`KismetMathLibrary.FInterpTo` (`self.CrystalVisibility`) 1.0 (`GameplayStatics.GetWorldDeltaSeconds`) 2.0)))
        (`KismetMaterialLibrary.SetScalarParameterValue` "/Game/Gameplay/Checkpoint/Param_Crystal.Param_Crystal" "Visibility" _output_get)
        (`SceneComponent.SetRelativeScale3D` (`self.NS_Crystal`) (`KismetMathLibrary.MakeVector` _output_get _output_get _output_get))
        (`SceneComponent.K2_SetRelativeRotation` (`self.Crystal`) (`KismetMathLibrary.ComposeRotators` (`KismetMathLibrary.MakeRotator` 0.0 0.0 (* (`GameplayStatics.GetWorldDeltaSeconds`) 50.0)) (`SceneComponent.RelativeRotation` (`self.Crystal`))) false false)
        (`SceneComponent.K2_SetRelativeLocation` (`self.Crystal`) (`KismetMathLibrary.VLerp` (`SceneComponent.RelativeLocation` (`self.Start`)) (`SceneComponent.RelativeLocation` (`self.End`)) (`self.CrystalVisibility`)) false false)
        (`LightComponent.SetIntensity` (`self.PointLight`) (`KismetMathLibrary.Lerp` 0.0 1.5 (`self.CrystalVisibility`)))))))

(event `self.Activate`
  (params (anInstigator :type "FPController Object Reference"))
  (bind _returnvalue (`FPController.GetFPCharacter` anInstigator))
  (bind _ns_pickupcrystal (`self.NS_PickupCrystal`))
  (`/Engine/EditorBlueprintResources/StandardMacros.IsValid` anInstigator
    (:`Is Valid`
      (set `self.Struck` true)
      (`SceneComponent.SetVisibility` _ns_pickupcrystal true false)
      (`ActorComponent.Activate` _ns_pickupcrystal true)
      (`FPTime.AddDilation` (`FPCharacter.myFPTime` _returnvalue) "CHECKPOINT" 1.0 -1.0 "/Game/Gameplay/Checkpoint/C_Dilation_Checkpoint.C_Dilation_Checkpoint")
      (`FPPostProcessing.SetPPScalar` (`FPCharacter.GetPostProcessing` _returnvalue) "PP_CRYSTAL" "Strength" 1.0 false)
      (`KismetSystemLibrary.Delay` 0.1)
      (`SceneComponent.SetVisibility` (`self.Crystal`) false false)
      (`SceneComponent.SetVisibility` (`self.NS_Crystal`) false false)
      (`KismetSystemLibrary.Delay` 0.2)
      (`self.FinishActivate` anInstigator))))

(event `self.OnEnable`
  (bind _ns_crystal (`self.NS_Crystal`))
  (`SceneComponent.SetVisibility` _ns_crystal true false)
  (`ActorComponent.Activate` _ns_crystal false)
  (`SceneComponent.SetVisibility` (`self.PointLight`) true false))

(fn `UserConstructionScript`)