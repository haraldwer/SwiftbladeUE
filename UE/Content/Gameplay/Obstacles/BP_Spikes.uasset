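; BP_Spikes is an obstacle that scatters instanced spike meshes over the surfaces inside its box.
; The construction script rebuilds the instances, with a count from box volume times Density, capped for safety.
; Each attempt picks a random point on the box footprint and traces down through the box on Visibility.
; Hits receive an instance with random cone tilt, spin and scale, oriented by Direction rather than the surface normal.
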(fn `Generate`
  (locals (Offset :type "Vector Structure") (TraceEnd :type "Vector Structure"))
  (bind _offset (`local.Offset`))
  (bind _returnvalue (`SceneComponent.K2_GetComponentLocation` (`self.Box`)))
  (bind _returnvalue_2 (`BoxComponent.GetScaledBoxExtent` (`self.Box`)))
  (bind _returnvalue_3 (`SceneComponent.GetUpVector` (`self.Box`)))
  (bind _z (.z (`BoxComponent.GetScaledBoxExtent` (`self.Box`))))
  (`InstancedStaticMeshComponent.ClearInstances` (`self.InstancedStaticMesh`))
  (`SceneComponent.SetAbsolute` (`self.InstancedStaticMesh`) false true true)
  (for _ (range (+ (`KismetMathLibrary.Min` (`KismetMathLibrary.FTrunc` (* (* (.x (* (`BoxComponent.GetScaledBoxExtent` (`self.Box`)) (`KismetMathLibrary.Conv_DoubleToVector` 0.01))) (.y (* (`BoxComponent.GetScaledBoxExtent` (`self.Box`)) (`KismetMathLibrary.Conv_DoubleToVector` 0.01))) (.z (* (`BoxComponent.GetScaledBoxExtent` (`self.Box`)) (`KismetMathLibrary.Conv_DoubleToVector` 0.01)))) (`self.Density`))) 1000) 1))
    (set `local.Offset` (+ (* (`KismetMathLibrary.RandomFloatInRange` (.x (* (`KismetMathLibrary.Conv_DoubleToVector` -1.0) _returnvalue_2)) (.x _returnvalue_2)) (`SceneComponent.GetForwardVector` (`self.Box`))) (* (`KismetMathLibrary.RandomFloatInRange` (.y (* (`KismetMathLibrary.Conv_DoubleToVector` -1.0) _returnvalue_2)) (.y _returnvalue_2)) (`SceneComponent.GetRightVector` (`self.Box`)))))
    (bind (_outhit _returnvalue_4) (`KismetSystemLibrary.LineTraceSingle` (+ _returnvalue _offset (* _z _returnvalue_3)) (+ _returnvalue _offset (* (* _z -1.0) _returnvalue_3)) "TraceTypeQuery1"))
    (if _returnvalue_4
      (`InstancedStaticMeshComponent.AddInstance` (`self.InstancedStaticMesh`) (`KismetMathLibrary.ComposeTransforms` (`KismetMathLibrary.MakeTransform` (0.0 0.0 0.0) (`KismetMathLibrary.ComposeRotators` (`KismetMathLibrary.Conv_VectorToRotator` (`KismetMathLibrary.RandomUnitVectorInConeInDegrees` (1.0 0.0 0.0) (`self.RandConeDeg`))) (`KismetMathLibrary.MakeRotator` 0.0 (`KismetMathLibrary.RandomFloatInRange` 0.0 360.0))) (`KismetMathLibrary.Conv_DoubleToVector` (`KismetMathLibrary.RandomFloatInRange` (`self.RandScaleMin`) (`self.RandScaleMax`)))) (`KismetMathLibrary.MakeTransform` (`.Location` (`GameplayStatics.BreakHitResult` _outhit)) (`KismetMathLibrary.ComposeRotators` (struct :`Roll` 90.0) (`KismetMathLibrary.Conv_VectorToRotator` (`self.Direction`))))) true))))

(fn `UserConstructionScript`
  (locals (NewLocalVar_0 :type "Float (double-precision)"))
  (`self.Generate`))