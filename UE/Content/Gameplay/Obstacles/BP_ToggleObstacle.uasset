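; BP_ToggleObstacle is an obstacle that alternates between enabled and disabled states on a timed, endless cycle.
; It starts disabled and waits a random time up to StartDuration before the first activation.
; A self-calling Update event then switches it on and off using delays of ActiveDuration and InactiveDuration.
; Enable and Disable events only set the Enabled flag, which IsEnabled exposes, with no visual or collision logic here.
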(event `self.ReceiveBeginPlay`
  (`self.Disable`)
  (`KismetSystemLibrary.Delay` (`KismetMathLibrary.RandomFloatInRange` 0.0 (`self.StartDuration`)))
  (`self.Update`))

(event `Update`
  (`self.Enable`)
  (`KismetSystemLibrary.Delay` (`self.ActiveDuration`))
  (`self.Disable`)
  (`KismetSystemLibrary.Delay` (`self.InactiveDuration`))
  (`self.Update`))

(event `Enable`
  (set `self.Enabled` true))

(event `Disable`
  (set `self.Enabled` false))

(fn `IsEnabled`
  (returns (Enabled :type Boolean))
  (return (`self.Enabled`)))

(fn `UserConstructionScript`)