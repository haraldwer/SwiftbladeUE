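; Obstacle that extends when enabled and retracts when disabled, hurting player characters it overlaps while extending.
; Enabling plays a Niagara twinkle, then after a delay shows the mesh and starts Tick, which moves Root between MeshStart and MeshEnd along separate extend and retract curves.
; Tick switches itself off at either end.
; Pawn collision is overlap during extension and block once extended; full retraction hides the mesh and disables its collision.
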(event `self.ReceiveBeginPlay`
  (`parent.ReceiveBeginPlay`)
  (`self.SetActorTickEnabled` false)
  (`SceneComponent.SetVisibility` (`self.NS_SharpTwinkle`) false false)
  (`SceneComponent.K2_SetRelativeTransform` (`self.Root`) (`SceneComponent.GetRelativeTransform` (`self.MeshStart`)) false false)
  (`self.Hide`))

(event `self.ReceiveTick`
  (params (DeltaSeconds :type "Float (single-precision)"))
  (bind _output_get (set `self.ExtendPart` (`KismetMathLibrary.FClamp` (+ (* DeltaSeconds (* (`self.ExtendSpeed`) (`KismetMathLibrary.SelectFloat` 1.0 -1.0 (`self.IsEnabled`)))) (`self.ExtendPart`)))))
  (`SceneComponent.K2_SetRelativeTransform` (`self.Root`) (`KismetMathLibrary.TLerp` (`SceneComponent.GetRelativeTransform` (`self.MeshStart`)) (`SceneComponent.GetRelativeTransform` (`self.MeshEnd`)) (`CurveFloat.GetFloatValue` (select `bool` (`self.IsEnabled`) :`false` (`self.RetractCurve`) :`true` (`self.ExtendCurve`)) _output_get)) false false)
  (if (`self.IsEnabled`)
    (`self.OnExtendTick` DeltaSeconds))
  (if (< (`KismetMathLibrary.Abs` (- (`self.ExtendPart`) (`KismetMathLibrary.Conv_BoolToDouble` (`self.IsEnabled`)))) 1e-05)
    (`self.SetActorTickEnabled` false)
    (if (`self.IsEnabled`)
      (`self.OnExtended`)
      (else
        (`self.Hide`)))))

(event `self.Enable`
  (`parent.Enable`)
  (`self.Twinkle`)
  (`KismetSystemLibrary.Delay` (`self.TwinkleDelay`))
  (`self.SetActorTickEnabled` true)
  (`self.Show`))

(event `self.Disable`
  (`parent.Disable`)
  (`self.SetActorTickEnabled` true))

(event `Twinkle`
  (`SceneComponent.SetVisibility` (`self.NS_SharpTwinkle`) true false)
  (`NiagaraComponent.ResetSystem` (`self.NS_SharpTwinkle`))
  (`KismetSystemLibrary.Delay` 2.0)
  (`SceneComponent.SetVisibility` (`self.NS_SharpTwinkle`) false false))

(event `Show`
  (bind _mesh (`self.Mesh`))
  (`/Engine/EditorBlueprintResources/StandardMacros.IsValid` _mesh
    (:`Is Valid`
      (`SceneComponent.SetVisibility` _mesh true false)
      (`PrimitiveComponent.SetCollisionEnabled` _mesh "QueryAndPhysics")
      (`PrimitiveComponent.SetCollisionResponseToChannel` _mesh "ECC_Pawn" "ECR_Overlap"))))

(event `Hide`
  (bind _mesh (`self.Mesh`))
  (`/Engine/EditorBlueprintResources/StandardMacros.IsValid` _mesh
    (:`Is Valid`
      (`SceneComponent.SetVisibility` _mesh false false)
      (`PrimitiveComponent.SetCollisionEnabled` _mesh "NoCollision"))))

(event `OnExtendTick`
  (params (DeltaTime :type "Float (double-precision)"))
  (bind _mesh (`self.Mesh`))
  (`/Engine/EditorBlueprintResources/StandardMacros.IsValid` _mesh
    (:`Is Valid`
      (for _array_element (`PrimitiveComponent.GetOverlappingActors` _mesh "/Game/Gameplay/Player/BP_FPCharacter.BP_FPCharacter_C")
        (`GameplayStatics.ApplyDamage` _array_element 1.0 null self "/Script/Engine.DamageType")))))

(event `OnExtended`
  (bind _mesh (`self.Mesh`))
  (`/Engine/EditorBlueprintResources/StandardMacros.IsValid` _mesh
    (:`Is Valid`
      (`PrimitiveComponent.SetCollisionResponseToChannel` _mesh "ECC_Pawn" "ECR_Block"))))

(fn `SetMesh`
  (params (Mesh :type "PrimitiveComponent Object Reference"))
  (set `self.Mesh` Mesh))

(fn `UserConstructionScript`
  (`parent.UserConstructionScript`))