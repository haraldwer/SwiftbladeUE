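; BP_SwingBlade is a swinging blade obstacle that damages the first-person player character on contact.
; Each tick it samples a looping float curve using game time, scaled by swing speed and amplitude, to set the blade's pitch.
; A random time offset chosen at BeginPlay varies the phase between instances.
; Four overlap boxes feed a shared DamagePlayer function, which applies damage only to BP_FPCharacter.
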(event `self.ReceiveBeginPlay`
  (set `self.TimeOffset` (`KismetMathLibrary.RandomFloat`)))

(event `self.ReceiveTick`
  (params (DeltaSeconds :type "Float (single-precision)"))
  (bind _swingcurve (`self.SwingCurve`))
  (`/Engine/EditorBlueprintResources/StandardMacros.IsValid` (`self.SwingCurve`)
    (:`Is Valid`
      (`SceneComponent.K2_SetRelativeRotation` (`self.Blade`) (`KismetMathLibrary.MakeRotator` 0.0 (* (`CurveFloat.GetFloatValue` _swingcurve (`KismetMathLibrary.FMod` (* (+ (`GameplayStatics.GetTimeSeconds`) (`self.TimeOffset`)) (`self.SwingSpeed`)) (`.MaxTime` (`CurveBase.GetTimeRange` _swingcurve)))) (`self.SwingAmount`))) false false))))

(event `self.Box.OnComponentBeginOverlap`
  (params (OverlappedComponent :type "PrimitiveComponent Object Reference") (OtherActor :type "Actor Object Reference") (OtherComp :type "PrimitiveComponent Object Reference") (OtherBodyIndex :type Integer) (bFromSweep :type Boolean) (SweepResult :type "HitResult Structure (by ref)"))
  (`self.DamagePlayer` OtherActor))

(event `self.Box1.OnComponentBeginOverlap`
  (params (OverlappedComponent :type "PrimitiveComponent Object Reference") (OtherActor :type "Actor Object Reference") (OtherComp :type "PrimitiveComponent Object Reference") (OtherBodyIndex :type Integer) (bFromSweep :type Boolean) (SweepResult :type "HitResult Structure (by ref)"))
  (`self.DamagePlayer` OtherActor))

(event `self.Box2.OnComponentBeginOverlap`
  (params (OverlappedComponent :type "PrimitiveComponent Object Reference") (OtherActor :type "Actor Object Reference") (OtherComp :type "PrimitiveComponent Object Reference") (OtherBodyIndex :type Integer) (bFromSweep :type Boolean) (SweepResult :type "HitResult Structure (by ref)"))
  (`self.DamagePlayer` OtherActor))

(event `self.Box3.OnComponentBeginOverlap`
  (params (OverlappedComponent :type "PrimitiveComponent Object Reference") (OtherActor :type "Actor Object Reference") (OtherComp :type "PrimitiveComponent Object Reference") (OtherBodyIndex :type Integer) (bFromSweep :type Boolean) (SweepResult :type "HitResult Structure (by ref)"))
  (`self.DamagePlayer` OtherActor))

(fn `DamagePlayer`
  (params (Object :type "Object Object Reference"))
  (bind _asbp_fpcharacter (cast `/Game/Gameplay/Player/BP_FPCharacter` Object))
  (`GameplayStatics.ApplyDamage` _asbp_fpcharacter 1.0 null self "/Script/Engine.DamageType"))

(fn `UserConstructionScript`)