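; Spinning blade obstacle that travels back and forth along a spline and damages the first-person player character on overlap.
; Each tick, a triangle wave of game time and MoveSpeed gives a target distance within padded spline ends, which FInterpTo smooths.
; Composed transforms layer time-based spin and roll onto the spline's local transform.
; A random time offset desynchronizes instances; Generate and the construction script do nothing.
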(event `self.ReceiveBeginPlay`
  (set `self.TimeOffset` (`KismetMathLibrary.RandomFloat`))
  (set `self.CurrentDistance` (`self.GetDesiredDistance`)))

(event `self.ReceiveTick`
  (params (DeltaSeconds :type "Float (single-precision)"))
  (`self.UpdateBlade` DeltaSeconds))

(event `self.Obstacle_SpinBlade.OnComponentBeginOverlap`
  (params (OverlappedComponent :type "PrimitiveComponent Object Reference") (OtherActor :type "Actor Object Reference") (OtherComp :type "PrimitiveComponent Object Reference") (OtherBodyIndex :type Integer) (bFromSweep :type Boolean) (SweepResult :type "HitResult Structure (by ref)"))
  (`self.DamagePlayer` OtherActor))

(fn `DamagePlayer`
  (params (Object :type "Object Object Reference"))
  (bind _asbp_fpcharacter (cast `/Game/Gameplay/Player/BP_FPCharacter` Object))
  (`GameplayStatics.ApplyDamage` _asbp_fpcharacter 1.0 null self "/Script/Engine.DamageType"))

(fn `Generate`)

(fn `GetDesiredDistance`
  (returns (ReturnValue :type "Float (double-precision)"))
  (bind _returnvalue (- (`SplineComponent.GetSplineLength` (`self.Spline`)) (* (`self.BladePadding`) 2.0)))
  (return (+ (`KismetMathLibrary.Abs` (- (`KismetMathLibrary.FMod` (* (`self.MoveSpeed`) (+ (`GameplayStatics.GetTimeSeconds`) (`self.TimeOffset`))) (* _returnvalue 2.0)) _returnvalue)) (`self.BladePadding`))))

(fn `UpdateBlade`
  (params (InputPin :type "Float (single-precision)"))
  (bind _output_get (set `self.DesiredDistance` (`self.GetDesiredDistance`)))
  (bind _output_get_2 (set `self.CurrentDistance` (`KismetMathLibrary.FInterpTo` (`self.CurrentDistance`) _output_get InputPin (`self.Smoothing`))))
  (`SceneComponent.K2_SetRelativeTransform` (`self.Obstacle_SpinBlade`) (`KismetMathLibrary.ComposeTransforms` (`KismetMathLibrary.MakeTransform` (0.0 0.0 0.0) (`KismetMathLibrary.MakeRotator` 0.0 0.0 (* (+ (`GameplayStatics.GetTimeSeconds`) (`self.TimeOffset`)) (`self.SpinSpeed`)))) (`KismetMathLibrary.ComposeTransforms` (`KismetMathLibrary.MakeTransform` (0.0 0.0 0.0) (`KismetMathLibrary.MakeRotator` (`self.Roll`))) (`SplineComponent.GetTransformAtDistanceAlongSpline` (`self.Spline`) _output_get_2 "Local" false))) false false))

(fn `UserConstructionScript`)