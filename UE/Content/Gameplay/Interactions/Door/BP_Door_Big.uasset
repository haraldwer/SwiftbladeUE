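; Big double door that swings open while the player interacts with it and swings back closed when interaction stops.
; Tick moves a clamped rotation toward open or closed based on the Interaction component's state, then smooths it and mirrors it onto both door leaves.
; Once the smoothed angle passes the finish offset, it notifies the local player a single time that the door opened.
; The bound Perform and Click handlers are empty.
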(event `self.ReceiveBeginPlay`
  (bind _interaction (`self.Interaction`))
  (add `Interaction.myOnPerformInteraction` _interaction (`|CreateDelegate` :!event `Perform`))
  (add `Interaction.myOnClickInteraction` _interaction (`|CreateDelegate` :!event `Click`)))

(event `Perform`
  (params (aCharacter :type "FPCharacter Object Reference")))

(event `Click`
  (params (aCharacter :type "FPCharacter Object Reference")))

(event `self.ReceiveTick`
  (params (DeltaSeconds :type "Float (single-precision)"))
  (bind _rotationspeed (`self.RotationSpeed`))
  (bind _output_get (set `self.Rotation` (`KismetMathLibrary.FClamp` (+ (`self.Rotation`) (* (* DeltaSeconds (`KismetMathLibrary.SelectFloat` (* _rotationspeed -1.0) _rotationspeed (`Interaction.IsInteracting` (`self.Interaction`)))) 1.0)) -70.0 0.0)))
  (bind _output_get_2 (set `self.SmoothRotation` (`KismetMathLibrary.FInterpTo` (`self.SmoothRotation`) _output_get DeltaSeconds (`self.Smoothing`))))
  (`SceneComponent.K2_SetRelativeRotation` (`self.Door_Big`) (`KismetMathLibrary.MakeRotator` 0.0 0.0 _output_get_2) false false)
  (`SceneComponent.K2_SetRelativeRotation` (`self.Door_Big1`) (`KismetMathLibrary.MakeRotator` 0.0 0.0 (+ (* _output_get_2 -1.0) 180.0)) false false)
  (if (< (`self.SmoothRotation`) (`self.FinishOffset`))
    (if (not (`self.Opened`))
      (bind _returnvalue (`MainSingelton.GetLocalPlayer`))
      (`/Engine/EditorBlueprintResources/StandardMacros.IsValid` _returnvalue
        (:`Is Valid`
          (`FPCharacter.DoorOpened` _returnvalue self)
          (set `self.Opened` true))))))

(fn `UserConstructionScript`)