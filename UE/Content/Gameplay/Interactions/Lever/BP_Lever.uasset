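; Interactable lever actor that is pulled down by click interaction and drifts back toward rest when released before completion.
; Interaction component events set the click state and enable Tick when interaction begins.
; Tick drives a clamped target pitch, faster pulling than returning, and eases the lever base toward it with FInterpTo.
; Nearing maximum rotation finishes the interaction, and the perform event disables Tick.
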(event `self.ReceiveBeginPlay`
  (bind _interaction (`self.Interaction`))
  (add `Interaction.myOnPerformInteraction` _interaction (`|CreateDelegate` :!event `OnPerform`))
  (add `Interaction.myOnClickInteraction` _interaction (`|CreateDelegate` :!event `OnClick`))
  (add `Interaction.myOnBeginInteract` _interaction (`|CreateDelegate` :!event `OnBeginInteract`))
  (add `Interaction.myOnEndInteract` _interaction (`|CreateDelegate` :!event `OnEndInteract`))
  (set `self.StartRotation` (`SceneComponent.RelativeRotation` (`self.LeverBase`)))
  (`self.SetActorTickEnabled` false))

(event `OnPerform`
  (params (aCharacter :type "FPCharacter Object Reference"))
  (`KismetSystemLibrary.PrintString` "Perform")
  (`self.SetActorTickEnabled` false))

(event `OnClick`
  (params (aCharacter :type "FPCharacter Object Reference"))
  (set `self.HasClicked` true))

(event `OnBeginInteract`
  (params (aCharacter :type "FPCharacter Object Reference"))
  (`self.SetActorTickEnabled` true))

(event `OnEndInteract`
  (params (aCharacter :type "FPCharacter Object Reference"))
  (set `self.HasClicked` false))

(event `self.ReceiveTick`
  (params (DeltaSeconds :type "Float (single-precision)"))
  (bind _output_get (set `self.CurrentRotation` (`KismetMathLibrary.FClamp` (+ (`self.CurrentRotation`) (* DeltaSeconds (`KismetMathLibrary.SelectFloat` -100.0 30.0 (and (`self.HasClicked`) (`Interaction.IsInteracting` (`self.Interaction`)))))) (`self.MaxRotation`) 0.0)))
  (bind _output_get_2 (set `self.SmoothRotation` (`KismetMathLibrary.FInterpTo` (`self.SmoothRotation`) _output_get DeltaSeconds 5.0)))
  ;[1 1 1] Set rot
  (`SceneComponent.K2_SetRelativeRotation` (`self.LeverBase`) (`KismetMathLibrary.ComposeRotators` (`KismetMathLibrary.MakeRotator` 0.0 _output_get_2) (`self.StartRotation`)) false false)
  ;[1 1 1] Check finish state
  (if (< (`KismetMathLibrary.Abs` (- (`self.SmoothRotation`) (`self.MaxRotation`))) 1.0)
    (`Interaction.FinishInteraction` (`self.Interaction`))))

(fn `UserConstructionScript`)