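; Stone platform variant that procedurally builds itself from a ring of randomly chosen meshes.
; Generate spaces pieces at equal angles, randomizing scale, yaw and height, with each piece's distance from the center scaled by its size.
; AddRandomMesh picks from the Meshes array and adds a local-space instance to the component returned by GetMeshComponent, avoiding a separate component per piece.
; The construction script only calls its parent.
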(fn `AddRandomMesh`
  (params (Transform :type "Transform Structure"))
  (bind _meshes (`self.Meshes`))
  (bind _component (`self.GetMeshComponent` (`|GetArrayItem` _meshes (`KismetMathLibrary.RandomIntegerInRange` 0 (- (`KismetArrayLibrary.Array_Length` _meshes) 1)))))
  (`/Engine/EditorBlueprintResources/StandardMacros.IsValid` _component
    (:`Is Valid`
      (`InstancedStaticMeshComponent.AddInstance` _component Transform false))))

(fn `Generate`
  (locals (Scale :type "Float (double-precision)"))
  (bind _heightoffset (`self.HeightOffset`))
  (for _index (range (`self.NumMeshes`))
    (set `local.Scale` (`KismetMathLibrary.RandomFloatInRange` (`self.MinSize`) (`self.MaxSize`)))
    (`self.AddRandomMesh` (`KismetMathLibrary.MakeTransform` (+ (* (`KismetMathLibrary.Conv_RotatorToVector` (`KismetMathLibrary.MakeRotator` 0.0 0.0 (* (`KismetMathLibrary.Conv_IntToDouble` _index) (/ 360 (`KismetMathLibrary.Conv_IntToDouble` (`self.NumMeshes`)))))) (* (`self.PositionOffset`) (`local.Scale`))) (`KismetMathLibrary.MakeVector` 0.0 0.0 (`KismetMathLibrary.RandomFloatInRange` (* _heightoffset -1.0) _heightoffset))) (`KismetMathLibrary.MakeRotator` 0.0 0.0 (`KismetMathLibrary.RandomFloatInRange` 0.0 360.0)) (`KismetMathLibrary.Conv_DoubleToVector` (`local.Scale`))))))

(fn `UserConstructionScript`
  (`parent.UserConstructionScript`))