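; First-person player character Blueprint that drives a speed-line effect from its movement.
; Each tick it normalizes movement velocity by max walk speed and writes to the Params_SpeedLines material parameter collection.
; Speed is an interpolated magnitude, squared and scaled by global time dilation.
; CenterOffset is an interpolated, halved velocity in camera space, so the effect's center follows movement relative to the view.
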(event `self.ReceiveTick`
  (params (DeltaSeconds :type "Float (single-precision)"))
  (`self.Update Speed Line Params`))

(fn `Update Speed Line Params`
  (bind _returnvalue (`GameplayStatics.GetWorldDeltaSeconds`))
  (bind _charactermovement (`self.CharacterMovement`))
  (bind _returnvalue_2 (/ (`CharacterMovementComponent.GetLastUpdateVelocity` _charactermovement) (`CharacterMovementComponent.MaxWalkSpeed` _charactermovement)))
  (`|ExecutionSequence`
    (:`then_0`
      (bind _output_get (set `self.SpeedSmoothing` (`KismetMathLibrary.FInterpTo` (`self.SpeedSmoothing`) (`KismetMathLibrary.FClamp` (* (/ (`KismetMathLibrary.VSize` _returnvalue_2) 1.0) 0.95)) _returnvalue 2.0)))
      (`KismetMaterialLibrary.SetScalarParameterValue` "/Game/Gameplay/Player/PostProcessing/Params_SpeedLines.Params_SpeedLines" "Speed" (* (`KismetMathLibrary.Square` _output_get) (`GameplayStatics.GetGlobalTimeDilation`))))
    (:`then_1`
      (bind _output_get_2 (set `self.DirectionSmoothing` (`KismetMathLibrary.VInterpTo` (`self.DirectionSmoothing`) (* (`KismetMathLibrary.InverseTransformDirection` (`SceneComponent.K2_GetComponentToWorld` (`self.myCamera`)) _returnvalue_2) (0.5 0.5 0.5)) _returnvalue 2.0)))
      (`KismetMaterialLibrary.SetVectorParameterValue` "/Game/Gameplay/Player/PostProcessing/Params_SpeedLines.Params_SpeedLines" "CenterOffset" (`KismetMathLibrary.Conv_VectorToLinearColor` _output_get_2)))))

(fn `UserConstructionScript`)