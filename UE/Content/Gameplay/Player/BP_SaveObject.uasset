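; BP_SaveObject stores a snapshot of first-person controller state, apparently for saving player progress.
; It holds arena index, in-arena flag, respawn count, seed and sword possession as separate variables.
; SetFromState unpacks an FPControllerState struct into those variables, and GetState rebuilds the struct from them.
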(fn `Get State`
  (returns (State :type "FPControllerState Structure"))
  (return (make `FPControllerState` (`self.ArenaIndex`) (`self.InArena`) (`self.RespawnCount`) (`self.Seed`) (`self.HasSword`))))

(fn `SetFromState`
  (params (State :type "FPControllerState Structure"))
  (bind (_myarenaindex _myinarena _myrespawncount _myseed _myhassword) (break `FPControllerState` State))
  (set `self.ArenaIndex` _myarenaindex)
  (set `self.InArena` _myinarena)
  (set `self.RespawnCount` _myrespawncount)
  (set `self.Seed` _myseed)
  (set `self.HasSword` _myhassword))