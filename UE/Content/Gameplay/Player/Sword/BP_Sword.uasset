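; The player's sword actor, with up to three magic crystals and a trail mesh.
; SetCrystalsActive toggles each changed crystal's point lights, can fire a Niagara effect on loss, and writes the count to Params_Sword after a short delay.
; Tick scales the trail by Params_Magic Strength and counters global time dilation on the mesh's Niagara effects.
; IntersectEffect is called each tick but does nothing, as its trace-driven spark logic is disconnected.
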(event `self.ReceiveTick`
  (params (DeltaSeconds :type "Float (single-precision)"))
  (`self.IntersectEffect`)
  (`self.ScaleTrailMesh`)
  (`self.FixStoneSparkDelta`))

(event `self.SetCrystalsActive`
  (params (aCrystalCount :type Integer) (aShowEffect :type Boolean))
  (bind _currentcrystalcount (`self.CurrentCrystalCount`))
  (bind _returnvalue (`KismetMathLibrary.Min` aCrystalCount _currentcrystalcount))
  (for _index (range _returnvalue (+ (`KismetMathLibrary.Max` aCrystalCount _currentcrystalcount) 1))
    (`self.Set Crystal Active` _index (< (`self.CurrentCrystalCount`) aCrystalCount) (and aShowEffect (== _returnvalue _index))))
  (bind _output_get (set `self.CurrentCrystalCount` aCrystalCount))
  (`KismetSystemLibrary.Delay` 0.09)
  (`KismetMaterialLibrary.SetScalarParameterValue` "/Game/Gameplay/Player/Sword/Params_Sword.Params_Sword" "CrystalCount" (`KismetMathLibrary.Conv_IntToDouble` _output_get)))

(fn `FixStoneSparkDelta`
  (for _array_element (`SceneComponent.GetChildrenComponents` (`self.Mesh`) true)
    (bind _asniagara_particle_system_component (cast `NiagaraComponent` _array_element))
    (`NiagaraComponent.SetCustomTimeDilation` _asniagara_particle_system_component (/ 1.0 (`GameplayStatics.GetGlobalTimeDilation`)))))

(fn `IntersectEffect`
  (locals (CachedPlayer :type "FPCharacter Object Reference")))

(fn `ScaleTrailMesh`
  (bind _returnvalue (`KismetMaterialLibrary.GetScalarParameterValue` "/Game/Gameplay/Player/PostProcessing/Params_Magic.Params_Magic" "Strength"))
  (`SceneComponent.SetRelativeScale3D` (`self.SwordTrail`) (`KismetMathLibrary.MakeVector` _returnvalue 1.0 1.0)))

(fn `Set Crystal Active`
  (params (Crystal :type Integer) (Active :type Boolean) (ShowParticle :type Boolean))
  (bind _returnvalue (select `int` Crystal :`0` (`self.Crystal_1`) :`1` (`self.Crystal_2`) :`2` (`self.Crystal_3`)))
  (`/Engine/EditorBlueprintResources/StandardMacros.IsValid` _returnvalue
    (:`Is Valid`
      (for _array_element (`SceneComponent.GetChildrenComponents` _returnvalue false)
        (bind _aspoint_light_component (cast `PointLightComponent` _array_element)
          (:`then`
            (`SceneComponent.SetVisibility` _aspoint_light_component Active false))
          (:`CastFailed`
            (bind _asniagara_particle_system_component (cast `NiagaraComponent` _array_element))
            (if (and ShowParticle (not Active))
              (`ActorComponent.Activate` _asniagara_particle_system_component true))))))))

(fn `UserConstructionScript`)