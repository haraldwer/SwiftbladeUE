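; BP_Grapple is a grapple point that shows when it is focused through a Niagara indicator, plane and point light.
; Focus begin and end events enable Tick, which interpolates a focus scale toward the focus state to grow or shrink the indicator and plane and fade the light.
; Tick is meant to switch off once settled, but its check compares against an offset target, so it generally keeps running.
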(event `self.ReceiveBeginPlay`
  (`NiagaraComponent.SetVariableFloat` (`self.NS_GrappleIndicator`) "b_Scale" 1.0)
  (`LightComponent.SetIntensity` (`self.PointLight`) 0.0)
  (`self.SetActorTickEnabled` false))

(event `self.OnBeginFocus`
  (`self.SetActorTickEnabled` true))

(event `self.OnEndFocus`
  (`self.SetActorTickEnabled` true))

(event `self.ReceiveTick`
  (params (DeltaSeconds :type "Float (single-precision)"))
  (bind _output_get (set `self.FocusScale` (`KismetMathLibrary.FInterpTo` (`self.FocusScale`) (`KismetMathLibrary.Conv_BoolToDouble` (`self.IsFocused`)) DeltaSeconds 10.0)))
  (bind _returnvalue (+ _output_get 1.0))
  (`NiagaraComponent.SetVariableFloat` (`self.NS_GrappleIndicator`) "b_Scale" _returnvalue)
  (`SceneComponent.SetRelativeScale3D` (`self.Plane`) (`KismetMathLibrary.Conv_DoubleToVector` _returnvalue))
  (`LightComponent.SetIntensity` (`self.PointLight`) (* _output_get 200.0))
  (if (< (`KismetMathLibrary.Abs` (- (`self.FocusScale`) (+ (`KismetMathLibrary.Conv_BoolToDouble` (`self.IsFocused`)) 1.0))) 0.001)
    (`self.SetActorTickEnabled` false)))

(fn `UserConstructionScript`)