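; Procedurally built wooden platform for the platform abilities, made of stacked layers of mesh instances.
; Generate calls GenerateLayer per layer, raising each by a fixed height and turning it about 90 degrees from the last for a crosshatched stack.
; GenerateMesh spreads instances across each layer with random offset, 180-degree flips, yaw and horizontal scale jitter, normalising scale to mesh size.
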(fn `Generate`
  (bind _component (`self.GetMeshComponent` (`self.Mesh`)))
  (`/Engine/EditorBlueprintResources/StandardMacros.IsValid` _component
    (:`Is Valid`
      (for _index (range (`self.NumLayers`))
        (`self.GenerateLayer` _index)))))

(fn `GenerateLayer`
  (params (LayerIndex :type Integer))
  (locals (LayerRot :type "Rotator Structure") (LayerPos :type "Vector Structure"))
  (bind _randlayerrot (`self.RandLayerRot`))
  (set `self.LayerYaw` (+ (+ (`self.LayerYaw`) (`KismetMathLibrary.RandomFloatInRange` (* _randlayerrot -1.0) _randlayerrot)) 90.0))
  (set `local.LayerRot` (`KismetMathLibrary.MakeRotator` 0.0 0.0 (`self.LayerYaw`)))
  (set `local.LayerPos` (`KismetMathLibrary.MakeVector` 0.0 0.0 (* (`self.LayerHeight`) (`local.LayerIndex`))))
  (for _index (range (`self.LayerNumMeshes`))
    (`self.GenerateMesh` _index (`local.LayerPos`) (`local.LayerRot`))))

(fn `GenerateMesh`
  (params (MeshIndex :type Integer) (LayerPos :type "Vector Structure") (LayerRot :type "Rotator Structure"))
  (bind _randrot (`self.RandRot`))
  (bind _randscale (`self.RandScale`))
  (bind _randoffsety (`self.RandOffsetY`))
  (bind _returnvalue (+ _randscale 1.0))
  (bind _returnvalue_2 (+ (* _randscale -1.0) 1.0))
  (bind _component (`self.GetMeshComponent` (`self.Mesh`)))
  (`/Engine/EditorBlueprintResources/StandardMacros.IsValid` _component
    (:`Is Valid`
      (`InstancedStaticMeshComponent.AddInstance` _component (`KismetMathLibrary.ComposeTransforms` (`KismetMathLibrary.MakeTransform` (+ (`local.LayerPos`) (`KismetMathLibrary.MakeVector` (`KismetMathLibrary.RandomFloatInRange` (* _randoffsety -1.0) _randoffsety) (- (* (`local.MeshIndex`) (/ (`self.RandOffsetX`) (`self.LayerNumMeshes`))) (* 0.5 (`self.RandOffsetX`))))) (`KismetMathLibrary.MakeRotator` (* (`KismetMathLibrary.Conv_BoolToDouble` (`KismetMathLibrary.RandomBool`)) 180.0) (* (`KismetMathLibrary.Conv_BoolToDouble` (`KismetMathLibrary.RandomBool`)) 180.0) (* (`KismetMathLibrary.Conv_BoolToDouble` (`KismetMathLibrary.RandomBool`)) 180.0)) (* (`self.AdjustScaleForMeshSize` (`self.Mesh`) (`self.Size`)) (`KismetMathLibrary.MakeVector` (`KismetMathLibrary.RandomFloatInRange` _returnvalue_2 _returnvalue) (`KismetMathLibrary.RandomFloatInRange` _returnvalue_2 _returnvalue) 1.0))) (`KismetMathLibrary.MakeTransform` (0.0 0.0 0.0) (`KismetMathLibrary.ComposeRotators` (`local.LayerRot`) (`KismetMathLibrary.MakeRotator` 0.0 0.0 (`KismetMathLibrary.RandomFloatInRange` (* _randrot -1.0) _randrot))))) false))))

(fn `UserConstructionScript`
  (`parent.UserConstructionScript`))