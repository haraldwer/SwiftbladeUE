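; Skull enemy Blueprint that adds a fiery visual reacting to movement and death on top of its parent enemy behavior.
; BeginPlay creates dynamic materials for the skull and fire, setting the skull's Strength to full.
; Tick normalizes and smooths velocity magnitude to drive the fire material's Strength.
; On death it hides the fire, then zeroes skull Strength and calls the parent handler only if that material is valid.
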(event `self.ReceiveBeginPlay`
  (`parent.ReceiveBeginPlay`)
  (bind _returnvalue (`PrimitiveComponent.CreateDynamicMaterialInstance` (`self.Fire`) 0 "/Game/Gameplay/Enemies/Types/Skull/M_Enemy_Skull_Fire.M_Enemy_Skull_Fire" "MI_Skull_Fire"))
  (set `self.FireMaterial` _returnvalue)
  (bind _returnvalue_2 (`PrimitiveComponent.CreateDynamicMaterialInstance` (`self.0_Skull`) 0 "/Game/Gameplay/Enemies/Types/Skull/M_Enemy_Skull.M_Enemy_Skull" "MI_Skull_Fire"))
  (bind _output_get (set `self.Material` _returnvalue_2))
  (`MaterialInstanceDynamic.SetScalarParameterValue` _output_get "Strength" 1.0))

(event `self.ReceiveTick`
  (params (DeltaSeconds :type "Float (single-precision)"))
  (`parent.ReceiveTick` DeltaSeconds)
  (bind _output_get (set `self.SmoothVel` (`KismetMathLibrary.FInterpTo` (`self.SmoothVel`) (`KismetMathLibrary.FClamp` (/ (`KismetMathLibrary.VSize` (`self.GetVelocity`)) 1000.0)) DeltaSeconds 5.0)))
  (`self.SetMaterialParam` _output_get))

(event `self.OnDied`
  (`SceneComponent.SetVisibility` (`self.Fire`) false false)
  (bind _material (`self.Material`)
    (:`then`
      (`MaterialInstanceDynamic.SetScalarParameterValue` _material "Strength" 0.0)
      (`parent.OnDied`))
    (:`else`)))

(fn `SetMaterialParam`
  (params (Strength :type "Float (double-precision)"))
  (bind _firematerial (`self.FireMaterial`)
    (:`then`
      (`MaterialInstanceDynamic.SetScalarParameterValue` _firematerial "Strength" Strength))
    (:`else`)))

(fn `UserConstructionScript`
  (`parent.UserConstructionScript`))