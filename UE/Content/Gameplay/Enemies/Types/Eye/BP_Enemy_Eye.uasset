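; Eye enemy with three spinning rings that act as a visual damage indicator.
; BeginPlay seeds a random stream for initial spins; Tick rotates each ring through RotateRing, which adds random drift damped toward zero by RInterpTo.
; The velocity Select is fixed at index 0, so all rings share and update the first velocity.
; Each hit destroys the last remaining ring, and death hides the eye, alongside parent handling.
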(event `self.ReceiveBeginPlay`
  (bind _rings (`self.Rings`))
  (bind _returnvalue (`KismetMathLibrary.MakeRotator` (`KismetMathLibrary.RandomFloatInRangeFromStream` -180.0 180.0 (`self.Random`)) (`KismetMathLibrary.RandomFloatInRangeFromStream` -180.0 180.0 (`self.Random`)) (`KismetMathLibrary.RandomFloatInRangeFromStream` -180.0 180.0 (`self.Random`))))
  (`parent.ReceiveBeginPlay`)
  (`KismetMathLibrary.SetRandomStreamSeed` (`self.Random`) (`KismetMathLibrary.RandomInteger` 9999999))
  (set `self.RingAngularVel_0` _returnvalue)
  (set `self.RingAngularVel_1` _returnvalue)
  (set `self.RingAngularVel_2` _returnvalue)
  (`KismetArrayLibrary.Array_Add` _rings (`self.Ring_0`))
  (`KismetArrayLibrary.Array_Add` _rings (`self.Ring_1`))
  (`KismetArrayLibrary.Array_Add` _rings (`self.Ring_2`)))

(event `self.ReceiveTick`
  (params (DeltaSeconds :type "Float (single-precision)"))
  (for _index (range (`KismetArrayLibrary.Array_Length` (`self.Rings`)))
    (`self.Rotate Ring` DeltaSeconds (`|GetArrayItem` (`self.Rings`) _index) (select `int` 0 :`0` (`self.RingAngularVel_0`) :`1` (`self.RingAngularVel_1`) :`2` (`self.RingAngularVel_2`)))))

(event `self.OnDied`
  (`SceneComponent.SetVisibility` (`self.Eye`) false false)
  (`parent.OnDied`))

(event `self.OnTookDamage`
  (params (aDamageAmount :type "Float (single-precision)") (aDamageCauser :type "Actor Object Reference"))
  (bind _rings (`self.Rings`))
  (bind _returnvalue (- (`KismetArrayLibrary.Array_Length` _rings) 1))
  (`parent.OnTookDamage` aDamageAmount aDamageCauser)
  (if (`KismetArrayLibrary.Array_IsNotEmpty` _rings)
    (`ActorComponent.K2_DestroyComponent` (`|GetArrayItem` (`self.Rings`) _returnvalue))
    (`KismetArrayLibrary.Array_Remove` (`self.Rings`) _returnvalue)))

(fn `Rotate Ring`
  (params (Delta :type "Float (double-precision)") (Ring :type "SceneComponent Object Reference") (Rotator :type "Rotator Structure (by ref)"))
  (`/Engine/EditorBlueprintResources/StandardMacros.IsValid` Ring
    (:`Is Valid`
      (`|VariableSetRef` Rotator (`KismetMathLibrary.RInterpTo` (`KismetMathLibrary.ComposeRotators` (* (`KismetMathLibrary.MakeRotator` (`KismetMathLibrary.RandomFloatInRangeFromStream` -180.0 180.0 (`self.Random`)) (`KismetMathLibrary.RandomFloatInRangeFromStream` -180.0 180.0 (`self.Random`)) (`KismetMathLibrary.RandomFloatInRangeFromStream` -180.0 180.0 (`self.Random`))) (* 1.0 Delta)) Rotator) (struct) Delta 0.05))
      (`SceneComponent.K2_AddWorldRotation` Ring (* Rotator Delta) false false))))

(fn `UserConstructionScript`
  (`parent.UserConstructionScript`))