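; Base enemy Blueprint that handles spawn, damage and death effects along with a dim, shadowless light.
; On BeginPlay it spawns a spawn particle, then hides the actor and pauses its actor and behaviour component ticks for a short delay before revealing and resuming it.
; Taking damage and dying both spawn the death particle, and death also breaks BPBreakable in a random direction.
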(event `self.ReceiveBeginPlay`
  (bind _light (`self.Light`))
  (`parent.ReceiveBeginPlay`)
  (`self.ShowSpawnEffect`)
  (`LightComponentBase.SetCastShadows` _light false)
  (`LocalLightComponent.SetAttenuationRadius` _light 500.0)
  (`LightComponent.SetIntensity` _light 0.2))

(event `ShowSpawnEffect`
  (`|SpawnActorFromClass` "/Game/Gameplay/Enemies/Effects/BP_Enemy_SpawnParticle.BP_Enemy_SpawnParticle_C" (`self.GetTransform`) "AlwaysSpawn" "OverrideRootScale" null null)
  (`self.SetActorHiddenInGame` true)
  (`self.SetActorTickEnabled` false)
  (`ActorComponent.SetComponentTickEnabled` (`self.myBehaviour`) false)
  (`KismetSystemLibrary.Delay` 1.7)
  (`self.SetActorHiddenInGame` false)
  (`self.SetActorTickEnabled` true)
  (`ActorComponent.SetComponentTickEnabled` (`self.myBehaviour`) true))

(event `self.OnDied`
  (`|SpawnActorFromClass` "/Game/Gameplay/Enemies/Effects/BP_Enemy_DeathParticle.BP_Enemy_DeathParticle_C" (`self.GetTransform`) "AlwaysSpawn" "OverrideRootScale" null null)
  (`Breakable.Break` (`self.BP_Breakable`) (`self.K2_GetActorLocation`) (`KismetMathLibrary.RandomUnitVector`)))

(event `self.OnTookDamage`
  (params (aDamageAmount :type "Float (single-precision)") (aDamageCauser :type "Actor Object Reference"))
  (`|SpawnActorFromClass` "/Game/Gameplay/Enemies/Effects/BP_Enemy_DeathParticle.BP_Enemy_DeathParticle_C" (`self.GetTransform`) "AlwaysSpawn" "OverrideRootScale" null null))

(fn `UserConstructionScript`)