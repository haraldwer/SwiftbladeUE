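; BP_Proc_Vines is a procedural vine prop that, as it stands, contains only debug scaffolding and generates no vines.
; The construction script traces forward from the actor by InitialRayLength on Visibility with persistent debug drawing, but nothing follows a hit.
; DrawSpline only flushes persistent debug lines and is not called here.
; Its disconnected loop would draw spheres and connecting lines along the Spline's points.
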(fn `DrawSpline`
  (locals (PreviousPoint :type "Vector Structure"))
  (`KismetSystemLibrary.FlushPersistentDebugLines`))

(fn `UserConstructionScript`
  (bind _returnvalue (`self.K2_GetActorLocation`))
  (bind (_outhit _returnvalue_2) (`KismetSystemLibrary.LineTraceSingle` :`Start` _returnvalue :`End` (+ _returnvalue (* (`self.GetActorForwardVector`) (`self.InitialRayLength`))) :`TraceChannel` "TraceTypeQuery1" :`bTraceComplex` true :`DrawDebugType` "Persistent"))
  (if _returnvalue_2
    _))