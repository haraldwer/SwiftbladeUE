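; BP_SliceMesh is a procedural helper actor that cuts a static mesh along a supplied set of edge planes.
; The construction script copies the mesh's first LOD0 section into a procedural mesh with material and blocking WorldStatic collision.
; Slice applies one planar cut per edge, capping into the last section, with the actor temporarily rescaled by pre and post multipliers.
; It then rebuilds the resulting first section with collision.
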(event `self.Slice`
  (params (someEdges :type "Array of SliceEdge Structure (by ref)"))
  (bind _result (`self.Result`))
  (`self.SetActorScale3D` (* (`self.GetActorScale3D`) (`self.PreScaleMultiplier`)))
  (for _array_element someEdges
    (bind (_mynormal _mylocation) (break `SliceEdge` _array_element))
    (`KismetProceduralMeshLibrary.SliceProceduralMesh` (`self.Result`) _mylocation _mynormal false "UseLastSectionForCap" (`self.Material`)))
  (`self.SetActorScale3D` (* (`self.GetActorScale3D`) (`self.PostScaleMultiplier`)))
  (bind (_vertices _triangles _normals _uvs _tangents) (`KismetProceduralMeshLibrary.GetSectionFromProceduralMesh` _result))
  (`ProceduralMeshComponent.CreateMeshSection_LinearColor` :`self` _result :`Vertices` _vertices :`Triangles` _triangles :`Normals` _normals :`UV0` _uvs :`Tangents` _tangents :`bCreateCollision` true))

(fn `UserConstructionScript`
  (bind _result (`self.Result`))
  (bind (_vertices _triangles _normals _uvs _tangents) (`KismetProceduralMeshLibrary.GetSectionFromStaticMesh` (`self.Mesh`)))
  (`ProceduralMeshComponent.CreateMeshSection_LinearColor` :`self` _result :`Vertices` _vertices :`Triangles` _triangles :`Normals` _normals :`UV0` _uvs :`Tangents` _tangents :`bCreateCollision` true)
  (`PrimitiveComponent.SetMaterial` _result 0 (`self.Material`))
  (`PrimitiveComponent.SetCollisionEnabled` _result "QueryAndPhysics")
  (`PrimitiveComponent.SetCollisionObjectType` _result "ECC_WorldStatic")
  (`PrimitiveComponent.SetCollisionResponseToAllChannels` _result "ECR_Block"))