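; Procedural floor prop that scatters random stone meshes inside a spline outline, rebuilt by the construction script.
; It computes padded bounds from the spline points, then samples seeded random positions at their mid height, with count set by area and density up to an iteration cap.
; A dot product against the nearest spline right vector keeps inside points.
; Each becomes a mesh instance with random scale and yaw, optionally height-adjusted by its bounds.
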(fn `Generate`
  (locals (MinPos :type "Vector Structure") (MaxPos :type "Vector Structure") (Iterations :type Integer) (TotalIterations :type Integer) (Pos :type "Vector Structure") (Scale :type "Float (double-precision)"))
  (bind _pos (`local.Pos`))
  (bind _spline (`self.Spline`))
  (bind _stream (`self.Stream`))
  (bind _returnvalue (`SplineComponent.GetNumberOfSplinePoints` (`self.Spline`)))
  (`self.ClearMeshComponents`)
  (if (> _returnvalue 0)
    (bind _output_get (set `local.MinPos` (`SplineComponent.GetLocationAtSplinePoint` (`self.Spline`) 0 "World")))
    (set `local.MaxPos` _output_get)
    (for _index (range (+ _returnvalue 1))
      (bind _returnvalue_2 (`SplineComponent.GetLocationAtSplinePoint` (`self.Spline`) _index "World"))
      (set `local.MinPos` (- (`KismetMathLibrary.MakeVector` (`KismetMathLibrary.FMin` (.x _returnvalue_2) (.x (`local.MinPos`))) (`KismetMathLibrary.FMin` (.y _returnvalue_2) (.y (`local.MinPos`))) (`KismetMathLibrary.FMin` (.z _returnvalue_2) (.z (`local.MinPos`)))) (`self.Padding`)))
      (set `local.MaxPos` (+ (`KismetMathLibrary.MakeVector` (`KismetMathLibrary.FMax` (.x _returnvalue_2) (.x (`local.MaxPos`))) (`KismetMathLibrary.FMax` (.y _returnvalue_2) (.y (`local.MaxPos`))) (`KismetMathLibrary.FMax` (.z _returnvalue_2) (.z (`local.MaxPos`)))) (`self.Padding`))))
    (set `local.Iterations` 0)
    (set `local.TotalIterations` (`KismetMathLibrary.FTrunc` (* (* (- (.x (`local.MaxPos`)) (.x (`local.MinPos`))) (- (.y (`local.MaxPos`)) (.y (`local.MinPos`)))) (`self.Density`))))
    (while (and (< (`local.Iterations`) (`self.MaxIterations`)) (< (`local.Iterations`) (`local.TotalIterations`)))
      (set `local.Iterations` (+ (`local.Iterations`) 1))
      (set `local.Pos` (`KismetMathLibrary.MakeVector` (`KismetMathLibrary.RandomFloatInRangeFromStream` (.x (`local.MinPos`)) (.x (`local.MaxPos`)) _stream) (`KismetMathLibrary.RandomFloatInRangeFromStream` (.y (`local.MinPos`)) (.y (`local.MaxPos`)) _stream) (* (+ (.z (`local.MinPos`)) (.z (`local.MaxPos`))) 0.5)))
      (if (< (`KismetMathLibrary.Dot_VectorVector` (`SplineComponent.FindRightVectorClosestToWorldLocation` _spline _pos "World") (- (`SplineComponent.FindLocationClosestToWorldLocation` _spline _pos "World") _pos)) 0.0)
        (bind _component (`self.GetMeshComponent` (`KismetArrayLibrary.Array_RandomFromStream` (`self.Meshes`) (`self.Stream`)) (`self.Spline`)))
        (`/Engine/EditorBlueprintResources/StandardMacros.IsValid` _component
          (:`Is Valid`
            (set `local.Scale` (`KismetMathLibrary.RandomFloatInRangeFromStream` (`self.StoneMinSize`) (`self.StoneMaxSize`) (`self.Stream`)))
            (bind (_min _max) (break `Box` (`StaticMesh.GetBoundingBox` (`StaticMeshComponent.StaticMesh` _component))))
            (`InstancedStaticMeshComponent.AddInstance` _component (`KismetMathLibrary.MakeTransform` (+ (`local.Pos`) (`KismetMathLibrary.MakeVector` 0.0 0.0 (* (* (* (.z (- _max _min)) (`local.Scale`)) 0.5) (`KismetMathLibrary.Conv_BoolToDouble` (`self.bAdjustZ`))))) (`KismetMathLibrary.MakeRotator` 0.0 0.0 (`KismetMathLibrary.RandomFloatInRangeFromStream` 0.0 360.0 (`self.Stream`))) (`KismetMathLibrary.Conv_DoubleToVector` (`local.Scale`))) true)))))))

(fn `UserConstructionScript`
  (locals (MinPos :type "Vector Structure") (MaxPos :type "Vector Structure") (Pos :type "Vector Structure") (Iterations :type Integer) (TotalIterations :type Integer) (Scale :type "Float (double-precision)"))
  (`self.Generate`))